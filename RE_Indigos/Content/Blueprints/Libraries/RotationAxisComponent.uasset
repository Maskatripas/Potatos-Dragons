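; A scene component that defines a rotation axis through its own orientation and supplies quarter-turn rotations around it.
; GibRotation returns a 90-degree rotator about the component's world up vector, with the sign picked by a Clockwise flag.
; GetClosest scans the direct child components and stores the one nearest a given location, along with its distance.
; BeginPlay caches the owning actor.
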(event Custom|Get%20Closest
  (params (Location :type Vector))
  (bind _children (Components|GetChildrenComponents false))
  (bind _returnvalue (Utilities|Array|LastIndex _children))
  (bind _output (Utilities|Array|Get(acopy) _children _returnvalue))
  (Variables|Default|SetClosestC _output)
  (Variables|Default|SetClosest (Math|Vector|VectorLength (- (Transformation|GetWorldLocation _output) Location)))
  (for _array_element _children
    (if (< (Math|Vector|VectorLength (- (Transformation|GetWorldLocation _array_element) Location)) (Variables|Default|GetClosest))
      (Variables|Default|SetClosestC _array_element)
      (Variables|Default|SetClosest (Math|Vector|VectorLength (- (Transformation|GetWorldLocation _array_element) Location))))))

(event EventBeginPlay
  (Variables|Default|SetOwner (Components|GetOwner)))

(fn GibRotation
  (params (Clockwise :type Boolean))
  (return (Math|Vector|RotatorfromAxisandAngle (Math|Vector|GetUpVector (Transformation|GetWorldRotation)) (Math|Float|SelectFloat 9e+01 -9e+01 Clockwise))))