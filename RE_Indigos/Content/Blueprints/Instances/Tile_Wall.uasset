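; Tile_Wall is a construction-script tool that builds a tiled wall from copies of one mesh as instances on an instanced mesh component.
; It applies the chosen mesh and material array, then expands the EmptyArray boxes into a unique list of grid cells to leave empty.
; It fills an X, Y, Z grid spaced by the mesh's bounding box size, skipping those cells to leave gaps.
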(event EventBeginPlay)

(event Collision|EventActorBeginOverlap
  (params (OtherActor :type Actor%20Object%20Reference)))

(event EventTick
  (params (DeltaSeconds :type Float%20%28single-precision%29)))

(fn ConstructionScript
  (bind _wall_staticmesh (Variables|Components|GetWall_StaticMesh))
  (bind _wall_instance (Variables|Default|GetWall_Instance))
  (bind _returnvalue (StaticMesh|GetBoundingBox _wall_staticmesh))
  (bind _returnvalue_2 (- (.max _returnvalue) (.min _returnvalue)))
  (Utilities|FlowControl|Sequence
    (:then_0
      (Components|StaticMesh|SetStaticMesh _wall_instance (Variables|Components|GetWall_StaticMesh))
      (for (_array_element _array_index) (Variables|Components|GetWall_Material)
        (Rendering|Material|SetMaterial _wall_instance _array_index _array_element)))
    (:then_1
      (for _array_element_2 (Variables|Default|GetEmptyArray)
        (for _index (range (.x (.min _array_element_2)) (.x (.max _array_element_2)))
          (for _index_2 (range (.y (.min _array_element_2)) (.y (.max _array_element_2)))
            (for _index_3 (range (.z (.min _array_element_2)) (.z (.max _array_element_2)))
              (Utilities|Array|AddUnique (LocalVariables|GetEmptyIndex) (Utilities|Struct|MakeIntVector _index _index_2 _index_3)))))))
    (:then_2
      (for _index_4 (range 0 (- (Variables|Default|GetNumX) 1))
        (for _index_5 (range 0 (- (Variables|Default|GetNumY) 1))
          (for _index_6 (range 0 (- (Variables|Default|GetNumZ) 1))
            (if (not (Utilities|Array|ContainsItem (LocalVariables|GetEmptyIndex) (Utilities|Struct|MakeIntVector _index_4 _index_5 _index_6)))
              (Components|InstancedStaticMesh|AddInstance (Variables|Default|GetWall_Instance) (Math|Transform|MakeTransform (Math|Vector|MakeVector (* _index_4 (.x _returnvalue_2)) (* _index_5 (.y _returnvalue_2)) (* _index_6 (.z _returnvalue_2))) "0, 0, 0" "1,1,1")))))))))