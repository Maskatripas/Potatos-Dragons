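; Construction-script actor that procedurally builds 3D grids of instanced meshes from each of its TileMaker_StaticMeshComponents.
; Each component's mesh is scaled from its bounds to the tile extent, rotated and offset by its bounds minimum.
; Per-component counts and spacing combine with global values, with an option to override extent-based spacing.
; Hole ranges, shifted down by one, expand into an exclusion list of skipped cells, using triple-loop macros.
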(event EventBeginPlay)

(event Collision|EventActorBeginOverlap
  (params (OtherActor :type Actor%20Object%20Reference)))

(event EventTick
  (params (DeltaSeconds :type Float%20%28single-precision%29)))

(fn ConstructionScript
  (Utilities|FlowControl|Sequence
    (:then_0
      (Rendering|SetVisibility (Variables|Default|GetRoot) (not (Variables|Components|GetHide%20Root)) false))
    (:then_1
      (for _array_element (Actor|GetComponentsByClass "/Game/Blueprints/Libraries/TileMaker_StaticMeshComponent.TileMaker_StaticMeshComponent_C")
        (bind _output_get (LocalVariables|SetTile%20Element _array_element))
        (Components|InstancedStaticMesh|ClearInstances _output_get)
        (Utilities|FlowControl|Sequence
          (:then_0
            ;[1 1 1] Build Exclusion Array
            (Utilities|Array|Clear (LocalVariables|GetTile%20Holes))
            (bind (_array_element_min _array_element_max) (Utilities|ForEachLoopV (Variables|/Game/Blueprints/Libraries/TileMaker_StaticMeshComponent.TileMaker_StaticMeshComponent_C|GetHoles (LocalVariables|GetTile%20Element)))
              (:Loop%20Body
                (bind _index (Utilities|TripleforLoop _array_element_min _array_element_max)
                  (:LoopBody
                    (Utilities|Array|AddUnique (LocalVariables|GetTile%20Holes) (- _index 1)))))))
          (:then_1
            ;[1 1 1] Tile Modification
            (bind _output_get_2 (LocalVariables|SetTile%20Rotation (Variables|/Game/Blueprints/Libraries/TileMaker_StaticMeshComponent.TileMaker_StaticMeshComponent_C|GetRotation (LocalVariables|GetTile%20Element))))
            (LocalVariables|SetTile%20Scale (/ (* (Variables|/Game/Blueprints/Libraries/TileMaker_StaticMeshComponent.TileMaker_StaticMeshComponent_C|GetExtent (LocalVariables|GetTile%20Element)) (Variables|/Script/Engine.SceneComponent|GetRelativeScale3D (LocalVariables|GetTile%20Element))) (- (.max (StaticMesh|GetBoundingBox (Variables|/Script/Engine.StaticMeshComponent|GetStaticMesh (LocalVariables|GetTile%20Element)))) (.min (StaticMesh|GetBoundingBox (Variables|/Script/Engine.StaticMeshComponent|GetStaticMesh (LocalVariables|GetTile%20Element)))))))
            (LocalVariables|SetScale%20Offset (Math|Vector|RotateVector (* (/ (* (Variables|/Game/Blueprints/Libraries/TileMaker_StaticMeshComponent.TileMaker_StaticMeshComponent_C|GetExtent (LocalVariables|GetTile%20Element)) (Variables|/Script/Engine.SceneComponent|GetRelativeScale3D (LocalVariables|GetTile%20Element))) (- (.max (StaticMesh|GetBoundingBox (Variables|/Script/Engine.StaticMeshComponent|GetStaticMesh (LocalVariables|GetTile%20Element)))) (.min (StaticMesh|GetBoundingBox (Variables|/Script/Engine.StaticMeshComponent|GetStaticMesh (LocalVariables|GetTile%20Element)))))) (.min (StaticMesh|GetBoundingBox (Variables|/Script/Engine.StaticMeshComponent|GetStaticMesh (LocalVariables|GetTile%20Element))))) _output_get_2)))
          (:then_2
            (bind _index_2 (Utilities|TripleforLoop :Last%20Index (- (* (Variables|/Game/Blueprints/Libraries/TileMaker_StaticMeshComponent.TileMaker_StaticMeshComponent_C|GetNumber (LocalVariables|GetTile%20Element)) (Variables|Default|GetGlobal%20Number)) 1))
              (:LoopBody
                (bind _output_get_3 (LocalVariables|SetTile%20Index _index_2))
                (if (not (Utilities|Array|ContainsItem (LocalVariables|GetTile%20Holes) _output_get_3))
                  (Components|InstancedStaticMesh|AddInstance (LocalVariables|GetTile%20Element) (Math|Transform|MakeTransform (+ (- (* (Utilities|AbsVector (Math|Vector|RotateVector (Variables|/Game/Blueprints/Libraries/TileMaker_StaticMeshComponent.TileMaker_StaticMeshComponent_C|GetExtent (LocalVariables|GetTile%20Element)) (LocalVariables|GetTile%20Rotation))) (Math|Vector|SelectVector "0, 0, 0" (LocalVariables|GetTile%20Index) (Variables|/Game/Blueprints/Libraries/TileMaker_StaticMeshComponent.TileMaker_StaticMeshComponent_C|GetOverride%20Spacing (LocalVariables|GetTile%20Element)))) (LocalVariables|GetScale%20Offset)) (+ (* (Variables|/Game/Blueprints/Libraries/TileMaker_StaticMeshComponent.TileMaker_StaticMeshComponent_C|GetSpacing_X (LocalVariables|GetTile%20Element)) (.x (LocalVariables|GetTile%20Index))) (* (Variables|/Game/Blueprints/Libraries/TileMaker_StaticMeshComponent.TileMaker_StaticMeshComponent_C|GetSpacing_Y (LocalVariables|GetTile%20Element)) (.y (LocalVariables|GetTile%20Index))) (* (Variables|/Game/Blueprints/Libraries/TileMaker_StaticMeshComponent.TileMaker_StaticMeshComponent_C|GetSpacing_Z (LocalVariables|GetTile%20Element)) (.z (LocalVariables|GetTile%20Index))) (* (Variables|Default|GetGlobal%20Spacing%20X) (.x (LocalVariables|GetTile%20Index))) (* (Variables|Default|GetGlobal%20Spacing%20Y) (.y (LocalVariables|GetTile%20Index))) (* (Variables|Default|GetGlobal%20Spacing%20Z) (.z (LocalVariables|GetTile%20Index))))) (LocalVariables|GetTile%20Rotation) (LocalVariables|GetTile%20Scale))))))))))))