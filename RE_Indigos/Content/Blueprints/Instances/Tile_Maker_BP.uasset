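; Tile Maker is a construction-script actor that builds a 3D grid of instanced tiles.
; Each Hierarchical Instanced Static Mesh component uses its first tag as an index into Tileset for extent, offset, spacing and rotation.
; Instances are scaled and pivot-corrected from mesh bounds to fit each cell.
; Cells inside EmptyArray ranges are skipped, and per-tile flags decide whether the last cell on each axis is filled.
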(event EventBeginPlay)

(event Collision|EventActorBeginOverlap
  (params (OtherActor :type Actor%20Object%20Reference)))

(event EventTick
  (params (DeltaSeconds :type Float%20%28single-precision%29)))

(fn ConstructionScript
  (bind _numy (Variables|Default|GetNumY))
  (bind _numz (Variables|Default|GetNumZ))
  (bind _numx (Variables|Default|GetNumX))
  (bind _tileset (Variables|Components|GetTileset))
  (bind _returnvalue (- _numy 1))
  (bind _returnvalue_2 (- _numz 1))
  (bind _returnvalue_3 (- _numx 1))
  (bind _output_get (LocalVariables|SetInstanceArray (Actor|GetComponentsByClass "/Script/Engine.HierarchicalInstancedStaticMeshComponent")))
  (if (!= (Utilities|Array|Length _output_get) (Utilities|Array|Length _tileset))
    (Utilities|Array|Resize _tileset (Utilities|Array|Length _output_get)))
  (for _array_element (LocalVariables|GetInstanceArray)
    (LocalVariables|SetTile%20Instance _array_element)
    (LocalVariables|SetTile%20Extent (.tileextent (Utilities|Array|Get(acopy) (Variables|Components|GetTileset) (Math|Conversions|ToInteger(Byte) (Utilities|String|ToString(Name) (Utilities|Array|Get(acopy) (Variables|/Script/Engine.ActorComponent|GetComponentTags _array_element)))))))
    (LocalVariables|SetTile%20Offset (.tileoffset (Utilities|Array|Get(acopy) (Variables|Components|GetTileset) (Math|Conversions|ToInteger(Byte) (Utilities|String|ToString(Name) (Utilities|Array|Get(acopy) (Variables|/Script/Engine.ActorComponent|GetComponentTags _array_element)))))))
    (LocalVariables|SetTile%20Spacing (.tilespacing (Utilities|Array|Get(acopy) (Variables|Components|GetTileset) (Math|Conversions|ToInteger(Byte) (Utilities|String|ToString(Name) (Utilities|Array|Get(acopy) (Variables|/Script/Engine.ActorComponent|GetComponentTags _array_element)))))))
    (LocalVariables|SetTile%20Rotation (.tilerotation (Utilities|Array|Get(acopy) (Variables|Components|GetTileset) (Math|Conversions|ToInteger(Byte) (Utilities|String|ToString(Name) (Utilities|Array|Get(acopy) (Variables|/Script/Engine.ActorComponent|GetComponentTags _array_element)))))))
    (LocalVariables|SetTile%20Last%20X (.lastx (Utilities|Array|Get(acopy) (Variables|Components|GetTileset) (Math|Conversions|ToInteger(Byte) (Utilities|String|ToString(Name) (Utilities|Array|Get(acopy) (Variables|/Script/Engine.ActorComponent|GetComponentTags _array_element)))))))
    (LocalVariables|SetTile%20Last%20Y (.lasty (Utilities|Array|Get(acopy) (Variables|Components|GetTileset) (Math|Conversions|ToInteger(Byte) (Utilities|String|ToString(Name) (Utilities|Array|Get(acopy) (Variables|/Script/Engine.ActorComponent|GetComponentTags _array_element)))))))
    (LocalVariables|SetTile%20Last%20Z (.lastz (Utilities|Array|Get(acopy) (Variables|Components|GetTileset) (Math|Conversions|ToInteger(Byte) (Utilities|String|ToString(Name) (Utilities|Array|Get(acopy) (Variables|/Script/Engine.ActorComponent|GetComponentTags _array_element)))))))
    (Utilities|FlowControl|Sequence
      (:then_0
        (Components|InstancedStaticMesh|ClearInstances (LocalVariables|GetTile%20Instance)))
      (:then_1
        (for _array_element_2 (Variables|Default|GetEmptyArray)
          (for _index (range (.x (.min _array_element_2)) (.x (.max _array_element_2)))
            (for _index_2 (range (.y (.min _array_element_2)) (.y (.max _array_element_2)))
              (for _index_3 (range (.z (.min _array_element_2)) (.z (.max _array_element_2)))
                (Utilities|Array|AddUnique (LocalVariables|GetEmptyIndex) (Utilities|Struct|MakeIntVector _index _index_2 _index_3)))))))
      (:then_2
        (for _index_4 (range 0 _returnvalue_3)
          (if (== _index_4 _returnvalue_3)
            (if (LocalVariables|GetTile%20Last%20X)
              (for _index_5 (range 0 _returnvalue) :!label _label
                (if (== _index_5 _returnvalue)
                  (if (LocalVariables|GetTile%20Last%20Y)
                    (for _index_6 (range 0 _returnvalue_2) :!label _label_2
                      (if (== _index_6 _returnvalue_2)
                        (if (LocalVariables|GetTile%20Last%20Z)
                          (if (not (Utilities|Array|ContainsItem (LocalVariables|GetEmptyIndex) (Utilities|Struct|MakeIntVector _index_4 _index_5 _index_6))) :!label _label_3
                            (Components|InstancedStaticMesh|AddInstance (LocalVariables|GetTile%20Instance) (Math|Transform|MakeTransform (+ (LocalVariables|GetTile%20Offset) (Math|Vector|MakeVector (* _index_4 (.X (Math|Vector|BreakVector (LocalVariables|GetTile%20Spacing)))) (* _index_5 (.Y (Math|Vector|BreakVector (LocalVariables|GetTile%20Spacing)))) (* _index_6 (.Z (Math|Vector|BreakVector (LocalVariables|GetTile%20Spacing))))) (- (Math|Vector|MakeVector (* _index_4 (Math|Float|Absolute(Float) (.X (Math|Vector|BreakVector (Math|Vector|RotateVector (LocalVariables|GetTile%20Extent) (LocalVariables|GetTile%20Rotation)))))) (* _index_5 (Math|Float|Absolute(Float) (.Y (Math|Vector|BreakVector (Math|Vector|RotateVector (LocalVariables|GetTile%20Extent) (LocalVariables|GetTile%20Rotation)))))) (* _index_6 (Math|Float|Absolute(Float) (.Z (Math|Vector|BreakVector (Math|Vector|RotateVector (LocalVariables|GetTile%20Extent) (LocalVariables|GetTile%20Rotation))))))) (Math|Vector|RotateVector (* (/ (* (LocalVariables|GetTile%20Extent) (Transformation|GetWorldScale (LocalVariables|GetTile%20Instance))) (- (.max (StaticMesh|GetBoundingBox (Variables|/Script/Engine.StaticMeshComponent|GetStaticMesh (LocalVariables|GetTile%20Instance)))) (.min (StaticMesh|GetBoundingBox (Variables|/Script/Engine.StaticMeshComponent|GetStaticMesh (LocalVariables|GetTile%20Instance)))))) (.min (StaticMesh|GetBoundingBox (Variables|/Script/Engine.StaticMeshComponent|GetStaticMesh (LocalVariables|GetTile%20Instance))))) (LocalVariables|GetTile%20Rotation)))) (LocalVariables|GetTile%20Rotation) (/ (* (LocalVariables|GetTile%20Extent) (Transformation|GetWorldScale (LocalVariables|GetTile%20Instance))) (- (.max (StaticMesh|GetBoundingBox (Variables|/Script/Engine.StaticMeshComponent|GetStaticMesh (LocalVariables|GetTile%20Instance)))) (.min (StaticMesh|GetBoundingBox (Variables|/Script/Engine.StaticMeshComponent|GetStaticMesh (LocalVariables|GetTile%20Instance))))))))))
                        (else
                          (goto _label_3)))))
                  (else
                    (goto _label_2)))))
            (else
              (goto _label))))))))