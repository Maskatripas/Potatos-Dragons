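; Conveyor belt actor that carries overlapping actors along its spline, with activator channels to toggle it on or off and to change Speed while flipping its direction indicator.
; Each tick it offsets tracked actors along the spline's nearest forward direction and messages those implementing the interact interface.
; Belts chain through ConveyerNext, yielding actors the next belt already holds.
; The construction script sets the back-link and joint materials.
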(event OnComponentBeginOverlap(ConveyerCollider)
  (params (OverlappedComponent :type Primitive%20Component%20Object%20Reference) (OtherActor :type Actor%20Object%20Reference) (OtherComp :type Primitive%20Component%20Object%20Reference) (OtherBodyIndex :type Integer) (bFromSweep :type Boolean) (SweepResult :type Hit%20Result%20Structure%20%28by%20ref%29))
  (Utilities|Array|AddUnique (Variables|Default|GetConveyerArray) OtherActor)
  (Class|InteractInterfaceBP|ToggleConveyer(Message) OtherActor self))

(event OnComponentEndOverlap(ConveyerCollider)
  (params (OverlappedComponent :type Primitive%20Component%20Object%20Reference) (OtherActor :type Actor%20Object%20Reference) (OtherComp :type Primitive%20Component%20Object%20Reference) (OtherBodyIndex :type Integer))
  (Utilities|Array|RemoveItem (Variables|Default|GetConveyerArray) OtherActor)
  (Class|InteractInterfaceBP|ToggleConveyer(Message) OtherActor))

(event EventTick
  (params (DeltaSeconds :type Float%20%28single-precision%29))
  (if (Variables|Default|GetOn)
    (for _array_element (Variables|Default|GetConveyerArray)
      (bind _conveyernext (Variables|Default|GetConveyerNext)
        (:then
          (if (not (Utilities|Array|ContainsItem (Variables|ConveyerBelt_BP_C|GetConveyerArray _conveyernext) _array_element))
            (Utilities|FlowControl|Sequence :!label _label
              (:then_0
                (Transformation|AddActorWorldOffset _array_element (* (Math|Vector|GetForwardVector (Class|SplineComponent|FindRotationClosesttoWorldLocation (Variables|Default|GetSpline) (Transformation|GetActorLocation _array_element) "World")) (* (Variables|Default|GetSpeed) DeltaSeconds)) true true))
              (:then_1
                (if (Utilities|DoesObjectImplementInterface _array_element "/Game/Blueprints/Libraries/Interfaces/Interact_Interface_BP.Interact_Interface_BP_C")
                  (Class|InteractInterfaceBP|ConveyerActivator(Message) _array_element self (* (Math|Vector|GetForwardVector (Class|SplineComponent|FindRotationClosesttoWorldLocation (Variables|Default|GetSpline) (Transformation|GetActorLocation _array_element) "World")) (* (Variables|Default|GetSpeed) DeltaSeconds)) "0, 0, 0"))))))
        (:else
          (goto _label))))))

(event EventTriggerActivator
  (params (Channel :type Integer))
  (switch int Channel
    (:0
      (bind _output_get (Variables|Default|SetOn (not (stale _output_get))))
      (Rendering|SetVisibility (Variables|Default|GetArrow) _output_get false))
    (:1
      (Math|Float|NegateFloat (Variables|Default|GetSpeed)
        (:%20%20
          (Transformation|AddRelativeRotation (Variables|Default|GetDirection) "0,180.000000, 0" false false))))))

(fn ConstructionScript
  (Utilities|FlowControl|Sequence
    (:then_0
      (bind _conveyernext (Variables|Default|GetConveyerNext)
        (:then
          (bind _output_get (Variables|ConveyerBelt_BP_C|SetConveyerPrev _conveyernext self))
          (Rendering|Material|SetMaterial (Variables|Default|GetNextBelt) 0 "/Game/Mannekins/Mixamo/Materials/Zbot_Joints_MAT.Zbot_Joints_MAT"))
        (:else)))
    (:then_1
      (Rendering|SetVisibility (Variables|Default|GetArrow) (Variables|Default|GetOn) true))))

(fn Interact
  (params (Telekinesis :type Boolean))
  (return false))