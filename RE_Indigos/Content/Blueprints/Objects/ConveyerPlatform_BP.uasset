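; Moving platform that carries overlapping actors between Path waypoint actors, starting at the first.
; An activator trigger, or a delayed overlap when Automatic, advances it one waypoint, looping around the array.
; The Conveyer timeline acts as a tick, stepping with VInterpToConstant until arrival.
; Each step also offsets tracked riders and sends movement deltas to those implementing Interact_Interface_BP.
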(event OnComponentBeginOverlap(ConveyerCollider)
  (params (OverlappedComponent :type Primitive%20Component%20Object%20Reference) (OtherActor :type Actor%20Object%20Reference) (OtherComp :type Primitive%20Component%20Object%20Reference) (OtherBodyIndex :type Integer) (bFromSweep :type Boolean) (SweepResult :type Hit%20Result%20Structure%20%28by%20ref%29))
  (Utilities|FlowControl|Sequence
    (:then_0
      (Utilities|Array|AddUnique (Variables|Default|GetConveyerArray) OtherActor)
      (Class|InteractInterfaceBP|ToggleConveyer(Message) self OtherActor))
    (:then_1
      (if (Variables|Default|GetAutomatic)
        (Utilities|FlowControl|Delay 0.3)
        (CallFunction|UP/Down)))))

(event OnComponentEndOverlap(ConveyerCollider)
  (params (OverlappedComponent :type Primitive%20Component%20Object%20Reference) (OtherActor :type Actor%20Object%20Reference) (OtherComp :type Primitive%20Component%20Object%20Reference) (OtherBodyIndex :type Integer))
  (Utilities|Array|RemoveItem (Variables|Default|GetConveyerArray) OtherActor)
  (Class|InteractInterfaceBP|ToggleConveyer(Message) OtherActor))

(event Custom|UP/Down
  (bind _returnvalue (Transformation|GetActorLocation))
  (bind _path (Variables|Default|GetPath))
  (if (not (Audio|Components|Audio|IsPlaying (Variables|Default|GetConveyer)))
    (Utilities|FlowControl|Sequence
      (:then_0
        (Math|Integer|IncrementInt (stale _output_get)))
      (:then_1
        (bind _output_get (Variables|Default|SetInit/End (Utilities|Modulo(integer) (stale _output_get) (Utilities|Array|Length _path))))
        (Variables|Default|SetTarget%20Location (Transformation|GetActorLocation (Utilities|Array|Get(acopy) _path _output_get)))
        (Timeline|Conveyer Play
          (:Update
            (if (Math|Vector|NotEqual(Vector) _returnvalue (Math|Interpolation|VInterptoConstant _returnvalue (Variables|Default|GetTarget%20Location) (Utilities|Time|GetWorldDeltaSeconds) (Variables|Default|GetSpeed)) 0.0001)
              (Transformation|AddActorWorldOffset (- (Math|Interpolation|VInterptoConstant _returnvalue (Variables|Default|GetTarget%20Location) (Utilities|Time|GetWorldDeltaSeconds) (Variables|Default|GetSpeed)) _returnvalue) true true)
              (for _array_element (Variables|Default|GetConveyerArray)
                (Utilities|FlowControl|Sequence
                  (:then_0
                    (Transformation|AddActorWorldOffset _array_element (- (Math|Interpolation|VInterptoConstant _returnvalue (Variables|Default|GetTarget%20Location) (Utilities|Time|GetWorldDeltaSeconds) (Variables|Default|GetSpeed)) _returnvalue) false true))
                  (:then_1
                    (if (Utilities|DoesObjectImplementInterface _array_element "/Game/Blueprints/Libraries/Interfaces/Interact_Interface_BP.Interact_Interface_BP_C")
                      (Class|InteractInterfaceBP|ConveyerActivator(Message) _array_element self (- (Math|Interpolation|VInterptoConstant _returnvalue (Variables|Default|GetTarget%20Location) (Utilities|Time|GetWorldDeltaSeconds) (Variables|Default|GetSpeed)) _returnvalue) "0, 0, 0")))))
              (else
                (Audio|Components|Audio|Stop (Variables|Default|GetConveyer))))))))))

(event EventTriggerActivator
  (params (Channel :type Integer))
  (CallFunction|UP/Down))

(fn ConstructionScript
  (Transformation|SetActorLocation (Transformation|GetActorLocation (Utilities|Array|Get(acopy) (Variables|Default|GetPath))) false false))

(fn Interact
  (params (Telekinesis :type Boolean))
  (return false))