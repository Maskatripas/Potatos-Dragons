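; TutorialObject_BP is a slowly spinning pickup-style object that shows tutorial text while the player character stands near it.
; When a MainChar_BP enters the collider, it creates a TutorialWidget_BP, fills it with three configurable text lines and adds it to the viewport.
; Overlapping characters are tracked in an array, so the widget is removed only once the last one leaves.
; Tick yaws the static mesh at a constant rate.
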(event OnComponentBeginOverlap(Collider)
  (params (OverlappedComponent :type Primitive%20Component%20Object%20Reference) (OtherActor :type Actor%20Object%20Reference) (OtherComp :type Primitive%20Component%20Object%20Reference) (OtherBodyIndex :type Integer) (bFromSweep :type Boolean) (SweepResult :type Hit%20Result%20Structure%20%28by%20ref%29))
  (bind _asmain_char_bp (Utilities|Casting|CastToMainChar_BP OtherActor))
  (Utilities|Array|AddUnique (Variables|Default|GetActiveActor) _asmain_char_bp)
  (Variables|Default|GetActiveWidget
    (:then)
    (:else
      (bind _returnvalue (UserInterface|CreateWidget "/Game/UI/TutorialWidget_BP.TutorialWidget_BP_C" (Game|GetPlayerController 0)))
      (bind _output_get (Variables|Default|SetActiveWidget _returnvalue))
      (Default|CreateText _output_get (Variables|Default|GetFirstLine) (Variables|Default|GetSecondLine) (Variables|Default|GetThirdLine))
      (UserInterface|Viewport|AddtoViewport _output_get 0))))

(event OnComponentEndOverlap(Collider)
  (params (OverlappedComponent :type Primitive%20Component%20Object%20Reference) (OtherActor :type Actor%20Object%20Reference) (OtherComp :type Primitive%20Component%20Object%20Reference) (OtherBodyIndex :type Integer))
  (bind _activeactor (Variables|Default|GetActiveActor))
  (bind _asmain_char_bp (Utilities|Casting|CastToMainChar_BP OtherActor))
  (Utilities|Array|RemoveItem _activeactor _asmain_char_bp)
  (Variables|Default|GetActiveWidget
    (:then
      (if (< (Utilities|Array|Length _activeactor) 1)
        (Widget|RemovefromParent (Variables|Default|GetActiveWidget))
        (Variables|Default|SetActiveWidget 0)))
    (:else)))

(event EventBeginPlay)

(event EventTick
  (params (DeltaSeconds :type Float%20%28single-precision%29))
  (Transformation|AddWorldRotation (Variables|Default|GetStaticMesh) (Math|Rotator|MakeRotator 0.0 0.0 (* DeltaSeconds 2e+01)) false false))

(fn ConstructionScript)