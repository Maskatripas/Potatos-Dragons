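; A switchable conveyor belt actor that carries pawns along a changeable direction.
; While on, Tick offsets every pawn overlapping AreaConveyer along that area's forward vector, scaled by Speed and delta time, without sweeping.
; TriggerActivator toggles the belt and its Direction indicator, whose scale the construction script compensates for actor scale.
; ChangeConveyerDirection rotates AreaConveyer to front, back, left or right relative to the rotation saved at construction.
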(event EventTick
  (params (DeltaSeconds :type Float%20%28single-precision%29))
  (if (Variables|Default|GetOn)
    ;[1 1 1] ConveyBeltSistem
    ;;[1 1 1] OffsetLoop
    (for _array_element (Collision|GetOverlappingActors (Variables|Default|GetAreaConveyer) "/Script/Engine.Pawn" :!class /Script/Engine.PrimitiveComponent)
      (Transformation|AddActorWorldOffset _array_element (* (Math|Vector|GetForwardVector (Transformation|GetWorldRotation (Variables|Default|GetAreaConveyer))) (* DeltaSeconds (Variables|Default|GetSpeed)))))))

(event EventTriggerActivator
  (params (Channel :type Integer))
  (bind _output_get (Variables|Default|SetOn (not (stale _output_get))))
  (Rendering|SetVisibility (Variables|Default|GetDirection) _output_get false))

(fn ConstructionScript
  ;[1 1 1] SetArrowDirectionScaleSoItDosentChange
  (Transformation|SetRelativeScale3D (Variables|Default|GetDirection) (/ "1.000000,1.000000,1.000000" (Transformation|GetActorScale3D)))
  ;[1 1 1] SetDefaultRotation
  (Variables|Default|SetDefaultRotation (Transformation|GetActorRotation))
  (Rendering|SetVisibility (Variables|Default|GetDirection) (Variables|Default|GetOn) false))

(fn ChangeConveyerDirection
  (params (NewDirection :type String))
  (bind _defaultrotation (Variables|Default|GetDefaultRotation))
  ;[1 1 1] SwitchTerminal
  (switch string NewDirection
    (:Default)
    (:Right
      ;[1 1 1] TurnConveyerToTheRight
      (Transformation|SetWorldRotation (Variables|Default|GetAreaConveyer) (Math|Rotator|CombineRotators (Variables|Default|GetDefaultRotation) "0,90.000000, 0") false false))
    (:Left
      ;[1 1 1] TurnConveyerToTheLeft
      (Transformation|SetWorldRotation (Variables|Default|GetAreaConveyer) (Math|Rotator|CombineRotators (Variables|Default|GetDefaultRotation) "0,-90.000000, 0") false false))
    (:Back
      ;[1 1 1] TurnConveyerToTheBack
      (Transformation|SetWorldRotation (Variables|Default|GetAreaConveyer) (Math|Rotator|CombineRotators _defaultrotation "0,180.000000, 0") false false))
    (:Front
      ;[1 1 1] TurnConveyerToTheFront(DefaultDirection)
      (Transformation|SetWorldRotation (Variables|Default|GetAreaConveyer) _defaultrotation false false))))

(fn Interact
  (params (Telekinesis :type Boolean))
  (return false))