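; ActivatorKey_BP is a spinning key pickup that unlocks linked activatable objects when the player interacts with it.
; A non-telekinesis Interact triggers Activate, which sends UnlockActivatorMessage to every entry in the Activables array and then destroys the key.
; Tick rotates the mesh by a Spin value, and ToggleWidget shows or hides the interaction prompt widget.
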(event Custom|Event%20Activate
  ;[1 1 1] Interface Events
  (for _array_element (Variables|Default|GetActivables)
    (Class|InteractInterfaceBP|UnlockActivator(Message) _array_element))
  (Actor|DestroyActor))

(event EventToggleWidget
  (params (Visible :type Boolean))
  ;[1 1 1] Interface Events
  (Rendering|SetVisibility (Variables|Default|GetInteractionWidget) Visible false))

(event EventTick
  (params (DeltaSeconds :type Float%20%28single-precision%29))
  ;[1 1 1] Spin Animation
  (Transformation|AddRelativeRotation (Variables|Default|GetActivatorMesh) (Variables|Default|GetSpin) false false))

(fn ConstructionScript)

(fn Interact
  (params (Telekinesis :type Boolean))
  (if (not Telekinesis)
    (CallFunction|EventActivate)
    (return false)))