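; GreenLight is a switchable spotlight actor with a LightCone component whose collision turns on and off with the light.
; The construction script copies X scale to Y, sets the spotlight's cone angle and radius through GetConeAngle, whose math uses LightCone bounds, and caches collision and intensity.
; It also applies the initial On state, and TriggerActivator flips that state by zeroing or restoring the cached values.
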(event EventTriggerActivator
  (bind _lightcone (Variables|Default|GetLightCone))
  (bind _spotlight (Variables|Default|GetSpotLight))
  (if (Variables|Default|GetOn)
    (Collision|SetCollisionEnabled _lightcone "NoCollision")
    (Rendering|Components|Light|SetIntensity _spotlight 0.0)
    (Variables|Default|SetOn false)
    (else
      (Collision|SetCollisionEnabled _lightcone (Variables|Default|GetCollision))
      (Rendering|Components|Light|SetIntensity _spotlight (Variables|Default|GetIntensity))
      (Variables|Default|SetOn true))))

(fn ConstructionScript
  (bind _returnvalue (Transformation|GetActorScale3D))
  (bind (_angle _radius) (|GetConeAngle))
  (bind _spotlight (Variables|Default|GetSpotLight))
  (bind _lightcone (Variables|Default|GetLightCone))
  (bind _spotlight_2 (Variables|Default|GetSpotLight))
  (Utilities|FlowControl|Sequence
    (:then_0
      (Transformation|SetActorScale3D (Math|Vector|MakeVector (.x _returnvalue) (.x _returnvalue) (.z _returnvalue)))
      (Rendering|Lighting|SetOuterConeAngle _spotlight _angle)
      (Rendering|Lighting|SetAttenuationRadius _spotlight _radius))
    (:then_1
      (Variables|Default|SetCollision (Collision|GetCollisionEnabled (Variables|Default|GetLightCone)))
      (Variables|Default|SetIntensity (Variables|/Script/Engine.LightComponentBase|GetIntensity (Variables|Default|GetSpotLight)))
      (if (Variables|Default|GetOn)
        (Collision|SetCollisionEnabled _lightcone (Variables|Default|GetCollision))
        (Rendering|Components|Light|SetIntensity _spotlight_2 (Variables|Default|GetIntensity))
        (else
          (Collision|SetCollisionEnabled _lightcone "NoCollision")
          (Rendering|Components|Light|SetIntensity _spotlight_2 0.0))))))