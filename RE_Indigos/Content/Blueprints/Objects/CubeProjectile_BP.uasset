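; CubeProjectile_BP is a cube projectile, apparently moved by telekinesis, that marks a teleport point where it hits.
; While its MovementActor is valid, Tick clears any teleport point and opens a gate.
; Box hits flag it as released and pass through that gate to spawn or move a TeleportTarget_BP to the cube's location.
; On destruction it sends Rafi a telekinesis cancel and removes the target.
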(event OnComponentHit(BoxComponent)
  (params (HitComponent :type Primitive%20Component%20Object%20Reference) (OtherActor :type Actor%20Object%20Reference) (OtherComp :type Primitive%20Component%20Object%20Reference) (NormalImpulse :type Vector :default "0, 0, 0") (Hit :type Hit%20Result%20Structure%20%28by%20ref%29))
  (bind _returnvalue (Transformation|GetActorLocation))
  (Variables|Default|SetReleased true)
  (Utilities|FlowControl|Gate false
    (:Exit
      (bind _teleportpoint (Variables|Default|GetTeleportPoint)
        (:then
          (Transformation|SetActorLocation _teleportpoint _returnvalue false true))
        (:else
          (bind _returnvalue_2 (Game|SpawnActorfromClass "/Game/Blueprints/Objects/TeleportTarget_BP.TeleportTarget_BP_C" (Math|Transform|MakeTransform _returnvalue "0, 0, 0" "1,1,1") "AlwaysSpawn" 0 (Variables|Default|GetInstigator)))
          (Variables|Default|SetTeleportPoint _returnvalue_2))))))

(event EventDestroyed
  (Utilities|FlowControl|Sequence
    (:then_0
      (bind _rafi (Variables|Default|GetRafi)
        (:then
          (Class|TelekinesisInterfaceBP|TelekinesisCancel(Message) _rafi))
        (:else)))
    (:then_1
      (bind _teleportpoint (Variables|Default|GetTeleportPoint)
        (:then
          (Actor|DestroyActor _teleportpoint))
        (:else)))))

(event EventTick
  (params (DeltaSeconds :type Float%20%28single-precision%29))
  (bind _returnvalue (Transformation|GetActorLocation))
  (Variables|Default|GetMovementActor
    (:then
      (Utilities|FlowControl|Sequence
        (:then_0
          (bind _teleportpoint (Variables|Default|GetTeleportPoint)
            (:then
              (Actor|DestroyActor _teleportpoint))
            (:else)))
        (:then_1
          (Utilities|FlowControl|Gate false) ; enters at Open
        )))
    (:else)))

(fn ConstructionScript)