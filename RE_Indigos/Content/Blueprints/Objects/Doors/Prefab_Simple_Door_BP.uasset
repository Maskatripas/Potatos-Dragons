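; Simple door prefab Blueprint that extends a parent door, adding shrinking collision and location-based opacity materials.
; ActivateDoor calls the parent, then uses Alpha to scale the collision root along X from full size to zero.
; The construction script derives two opposite world-space corners from the rotated DoorOccluder box.
; It feeds them as bounds to dynamic white, black, glass and floor-light LocBasedOpacity materials on the door mesh.
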(event EventActivateDoor
  (params (Alpha :type Float%20%28single-precision%29))
  (|CallParentFunction Alpha)
  (Transformation|SetRelativeScale3D (Variables|Default|GetDoorCollisionRoot) (Math|Vector|Lerp(Vector) "1.000000,1.000000,1.000000" "0.000000,1.000000,1.000000" Alpha)))

(fn ConstructionScript
  (bind _dooroccluder (Variables|Default|GetDoorOccluder))
  (bind _sm_simpledoor_2x2_001_doorsimple (Variables|Default|GetSM_SimpleDoor_2x2_001_Doorsimple))
  (bind _returnvalue (Transformation|GetWorldLocation _dooroccluder))
  (bind _returnvalue_2 (Transformation|GetWorldRotation _dooroccluder))
  (bind _returnvalue_3 (Components|Box|GetScaledBoxExtent _dooroccluder))
  (bind _returnvalue_4 (Math|Vector|RotateVector _returnvalue_3 _returnvalue_2))
  (|CallParentFunction)
  (LocalVariables|SetOccluderPositive (Math|Conversions|ToLinearColor(Vector) (+ _returnvalue _returnvalue_4)))
  (LocalVariables|SetOccluderNegative (Math|Conversions|ToLinearColor(Vector) (- _returnvalue _returnvalue_4)))
  (Utilities|FlowControl|Sequence
    (:then_0
      (bind _returnvalue_5 (Rendering|Material|CreateDynamicMaterialInstance _sm_simpledoor_2x2_001_doorsimple 0 "/Game/Arte/Materials/OpacityMaterials/LocBasedOpacity_Material_White.LocBasedOpacity_Material_White" :!class /Script/Engine.PrimitiveComponent))
      (Utilities|FlowControl|Sequence
        (:then_0
          (Rendering|Material|SetVectorParameterValue _returnvalue_5 "Positive Bounds" (LocalVariables|GetOccluderPositive) :!class /Script/Engine.MaterialInstanceDynamic))
        (:then_1
          (Rendering|Material|SetVectorParameterValue _returnvalue_5 "Negative Bounds" (LocalVariables|GetOccluderNegative) :!class /Script/Engine.MaterialInstanceDynamic))))
    (:then_1
      (bind _returnvalue_6 (Rendering|Material|CreateDynamicMaterialInstance _sm_simpledoor_2x2_001_doorsimple 1 "/Game/Arte/Materials/OpacityMaterials/LocBasedOpacity_Material_Black.LocBasedOpacity_Material_Black" :!class /Script/Engine.PrimitiveComponent))
      (Utilities|FlowControl|Sequence
        (:then_0
          (Rendering|Material|SetVectorParameterValue _returnvalue_6 "Positive Bounds" (LocalVariables|GetOccluderPositive) :!class /Script/Engine.MaterialInstanceDynamic))
        (:then_1
          (Rendering|Material|SetVectorParameterValue _returnvalue_6 "Negative Bounds" (LocalVariables|GetOccluderNegative) :!class /Script/Engine.MaterialInstanceDynamic))))
    (:then_2
      (bind _returnvalue_7 (Rendering|Material|CreateDynamicMaterialInstance _sm_simpledoor_2x2_001_doorsimple 2 "/Game/Arte/Materials/OpacityMaterials/LocBasedOpacity_Material_Glass.LocBasedOpacity_Material_Glass" :!class /Script/Engine.PrimitiveComponent))
      (Utilities|FlowControl|Sequence
        (:then_0
          (Rendering|Material|SetVectorParameterValue _returnvalue_7 "Positive Bounds" (LocalVariables|GetOccluderPositive) :!class /Script/Engine.MaterialInstanceDynamic))
        (:then_1
          (Rendering|Material|SetVectorParameterValue _returnvalue_7 "Negative Bounds" (LocalVariables|GetOccluderNegative) :!class /Script/Engine.MaterialInstanceDynamic))))
    (:then_3
      (bind _returnvalue_8 (Rendering|Material|CreateDynamicMaterialInstance _sm_simpledoor_2x2_001_doorsimple 3 "/Game/Arte/Materials/OpacityMaterials/LocBasedOpacity_Material_FloorLight.LocBasedOpacity_Material_FloorLight" :!class /Script/Engine.PrimitiveComponent))
      (Utilities|FlowControl|Sequence
        (:then_0
          (Rendering|Material|SetVectorParameterValue _returnvalue_8 "Positive Bounds" (LocalVariables|GetOccluderPositive) :!class /Script/Engine.MaterialInstanceDynamic))
        (:then_1
          (Rendering|Material|SetVectorParameterValue _returnvalue_8 "Negative Bounds" (LocalVariables|GetOccluderNegative) :!class /Script/Engine.MaterialInstanceDynamic))))))