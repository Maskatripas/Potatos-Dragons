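; Concept door prefab that extends a parent door Blueprint with a visible lock indicator.
; Its UnlockDoor override calls the parent, then teleports the lock mesh to one of two points on the Lock spline according to the Locked flag.
; It also toggles the locked and unlocked lights so only the one matching the current state shows.
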(event EventUnlockDoor
  (params (Locked :type Boolean))
  (bind _returnvalue (not Locked))
  (|CallParentFunction Locked)
  (Utilities|FlowControl|Sequence
    (:then_0
      (Transformation|SetRelativeLocation (Variables|Default|GetLockMesh) (Spline|GetLocationatSplinePoint (Variables|Default|GetLock) (Math|Conversions|ToInteger(Boolean) _returnvalue) "Local") false true))
    (:then_1
      (Rendering|SetVisibility (Variables|Default|GetLockLight_Unlocked) _returnvalue false))
    (:then_2
      (Rendering|SetVisibility (Variables|Default|GetLockLight_Locked) Locked false))))

(fn ConstructionScript
  (|CallParentFunction))