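; Base door Blueprint that opens and closes through interaction or activator triggers, with optional locking.
; A timeline plays or reverses by Closed state, sliding tagged DoorPanel children between the first two points of their DoorPath splines.
; Triggers bypass the lock, while UnlockActivator toggles it and calls the empty UnlockDoor hook.
; The construction script applies initial state, and a retriggerable delay hides the interaction prompt.
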(event Custom|Event%20Activate
  ;[1 1 1] Interface Events
  (if (not (Variables|Default|GetLocked))
    (if (not (Audio|Components|Audio|IsPlaying (Variables|Default|GetDoor%20Movement)))
      (if (Variables|Default|GetClosed)
        (bind _alpha (Timeline|Door%20Movement PlayFromStart)
          (:Update
            (CallFunction|ActivateDoor _alpha))
          (:Finished
            (bind _output_get (Variables|Default|SetClosed (not (stale _output_get))))))
        (else
          (Timeline|Door%20Movement ReverseFromEnd))))))

(event EventTriggerActivator
  (params (Channel :type Integer))
  ;[1 1 1] Interface Events
  (if (not (Audio|Components|Audio|IsPlaying (Variables|Default|GetDoor%20Movement)))
    (if (Variables|Default|GetClosed)
      (bind _alpha (Timeline|Door%20Movement PlayFromStart)
        (:Update
          (CallFunction|ActivateDoor _alpha))
        (:Finished
          (bind _output_get (Variables|Default|SetClosed (not (stale _output_get))))))
      (else
        (Timeline|Door%20Movement ReverseFromEnd)))))

(event EventUnlockActivator
  ;[1 1 1] Interface Events
  (bind _output_get (Variables|Default|SetLocked (not (stale _output_get))))
  (CallFunction|UnlockDoor _output_get))

(event EventToggleWidget
  ;[1 1 1] Interface Events
  (if (not (Variables|Default|GetLocked))
    (Rendering|SetVisibility (Variables|Default|GetInteractionWidget) true false)
    (Utilities|FlowControl|RetriggerableDelay 0.2)
    (Rendering|SetVisibility (Variables|Default|GetInteractionWidget) false false)))

(fn ConstructionScript
  (Utilities|FlowControl|Sequence
    (:then_0
      (CallFunction|UnlockDoor (Variables|Default|GetLocked)))
    (:then_1
      (if (not (Variables|Default|GetClosed))
        (CallFunction|ActivateDoor 1.0)))))

(fn ActivateDoor
  (params (Alpha :type Float%20%28single-precision%29))
  (for _array_element (Actor|GetComponentsbyTag "/Script/Engine.SplineComponent" "DoorPath")
    (for _array_element_2 (Components|GetChildrenComponents _array_element false)
      (if (Components|ComponentHasTag _array_element_2 "DoorPanel")
        (Transformation|SetRelativeLocation _array_element_2 (Math|Vector|Lerp(Vector) (Spline|GetLocationatSplinePoint _array_element 0 "Local") (Spline|GetLocationatSplinePoint _array_element 1 "Local") Alpha) false true)))))

(fn UnlockDoor
  (params (Locked :type Boolean)))

(fn Interact
  (params (Telekinesis :type Boolean))
  (if (not Telekinesis)
    (CallFunction|EventActivate)
    (return false)))