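; Interactable trigger that, when used directly or via optional telekinesis, sends its Channel message to every linked Activable.
; Hold mode messages on each toggle and again if telekinesis ends while held; it overrides SingleUse, which otherwise locks the trigger after one activation.
; Retriggerable delays keep the interaction widget and channel-stencilled custom depth highlight visible only while their update events keep arriving.
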(event Custom|Event%20Activate
  ;[1 1 1] Interface Events
  (if (Variables|Default|GetHold)
    (bind _output_get (Variables|Default|SetHolding (not (stale _output_get))))
    (elif (Variables|Default|GetSingle%20Use)
      (Utilities|FlowControl|DoOnce false
        (:Completed
          (Variables|Default|SetLocked true)))))
  (for _array_element (Variables|Default|GetActivables)
    (Class|InteractInterfaceBP|TriggerActivator(Message) _array_element (Variables|Default|GetChannel))))

(event EventToggleWidget
  ;[1 1 1] Interface Events
  (if (not (Variables|Default|GetLocked))
    (Rendering|SetVisibility (Variables|Default|GetInteractionWidget) true false)
    (Utilities|FlowControl|RetriggerableDelay 0.2)
    (Rendering|SetVisibility (Variables|Default|GetInteractionWidget) false false)))

(event EventTelekinesisEffectUpdate
  (params (Channel :type Integer))
  (bind _variable (|TemporaryVariable))
  (bind _activatormesh_base (Variables|Default|GetActivatorMesh_Base))
  ;[1 1 1] Interface Events
  (Utilities|FlowControl|Sequence
    (:then_0
      (if (!= Channel _variable)
        (goto _label Reset)))
    (:then_1
      (Utilities|FlowControl|DoOnce false :!label _label
        (:Completed
          (Rendering|SetRenderCustomDepth _activatormesh_base true)
          (Rendering|SetCustomDepthStencilValue _activatormesh_base Channel)
          (|Assign _variable Channel))))
    (:then_2
      (Utilities|FlowControl|RetriggerableDelay 0.3)
      (Rendering|SetRenderCustomDepth (Variables|Default|GetActivatorMesh_Base) false)
      (goto _label Reset))))

(event EventTelekinesisBegin
  (params (Rafi :type Pawn%20Object%20Reference) (H%20range :type Float%20%28single-precision%29) (V%20Range :type Float%20%28single-precision%29))
  ;[1 1 1] Interface Events
  (Variables|Default|SetRafi Rafi))

(event EventTelekinesisEnd
  (params (Rafi :type Pawn%20Object%20Reference))
  ;[1 1 1] Interface Events
  (Variables|Default|SetRafi 0)
  (if (Variables|Default|GetHolding)
    (Variables|Default|SetHolding false)
    (for _array_element (Variables|Default|GetActivables)
      (Class|InteractInterfaceBP|TriggerActivator(Message) _array_element (Variables|Default|GetChannel)))))

(fn ConstructionScript
  (bind _telekinesiscomponent (Variables|Default|GetTelekinesisComponent))
  (Utilities|FlowControl|Sequence
    (:then_0
      (if (Variables|Default|GetTelekinesis)
        (Collision|SetCollisionEnabled _telekinesiscomponent "QueryOnly")
        (else
          (Collision|SetCollisionEnabled _telekinesiscomponent "NoCollision"))))
    (:then_1
      (if (Variables|Default|GetHold)
        (Variables|Default|SetSingle%20Use false)))))

(fn Interact
  (params (Telekinesis :type Boolean))
  (if Telekinesis
    (if (Variables|Default|GetTelekinesis)
      (CallFunction|EventActivate :!label _label)
      (return (Variables|Default|GetHold)))
    (else
      (goto _label))))

(fn TelekinesisCameraOffset
  (return 0.0))

(fn TelekinesisPileUp
  (params (Input :type Array%20of%20Actor%20Object%20References))
  (return 0))