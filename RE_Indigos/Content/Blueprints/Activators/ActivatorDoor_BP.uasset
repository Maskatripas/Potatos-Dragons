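; Activator door with two panels that opens and closes when triggered or interacted with, with a lock that blocks interaction until unlocked.
; Trigger bypasses the lock and shares a DoOnce with interaction, ignoring new requests until the movement finishes.
; A timeline lerps each panel's relative location and scale, playing forward or in reverse based on the Closed flag, which flips on finish.
; The construction script places panels in the open pose when Closed is false.
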(event EventUnlockActivator
  (Variables|Default|SetLocked false))

(event EventTriggerActivator
  (bind _door1 (Variables|Default|GetDoor1))
  (bind _door2 (Variables|Default|GetDoor2))
  (Utilities|FlowControl|DoOnce false :!label _label
    (:Completed
      (if (Variables|Default|GetClosed)
        (bind _alpha (Timeline|Door%20Movement PlayFromStart)
          (:Update
            (Transformation|SetRelativeLocation _door1 (Math|Vector|Lerp(Vector) "0, 0,50.000000" (Variables|Default|GetDoorPosition1) _alpha) false false)
            (Transformation|SetRelativeScale3D _door1 (Math|Vector|Lerp(Vector) "1.000000,1.000000,1.000000" (Variables|Default|GetDoorScale) _alpha))
            (Transformation|SetRelativeLocation _door2 (Math|Vector|Lerp(Vector) "0, 0,150.000000" (Variables|Default|GetDoorPosition2) _alpha) false false)
            (Transformation|SetRelativeScale3D _door2 (Math|Vector|Lerp(Vector) "1.000000,1.000000,1.000000" (Variables|Default|GetDoorScale) _alpha)))
          (:Finished
            (bind _output_get (Variables|Default|SetClosed (not (stale _output_get))))
            (goto _label Reset)))
        (else
          (Timeline|Door%20Movement ReverseFromEnd))))))

(event EventInteractActivator
  (bind _door1 (Variables|Default|GetDoor1))
  (bind _door2 (Variables|Default|GetDoor2))
  (if (not (Variables|Default|GetLocked))
    (Utilities|FlowControl|DoOnce false :!label _label
      (:Completed
        (if (Variables|Default|GetClosed)
          (bind _alpha (Timeline|Door%20Movement PlayFromStart)
            (:Update
              (Transformation|SetRelativeLocation _door1 (Math|Vector|Lerp(Vector) "0, 0,50.000000" (Variables|Default|GetDoorPosition1) _alpha) false false)
              (Transformation|SetRelativeScale3D _door1 (Math|Vector|Lerp(Vector) "1.000000,1.000000,1.000000" (Variables|Default|GetDoorScale) _alpha))
              (Transformation|SetRelativeLocation _door2 (Math|Vector|Lerp(Vector) "0, 0,150.000000" (Variables|Default|GetDoorPosition2) _alpha) false false)
              (Transformation|SetRelativeScale3D _door2 (Math|Vector|Lerp(Vector) "1.000000,1.000000,1.000000" (Variables|Default|GetDoorScale) _alpha)))
            (:Finished
              (bind _output_get (Variables|Default|SetClosed (not (stale _output_get))))
              (goto _label Reset)))
          (else
            (Timeline|Door%20Movement ReverseFromEnd)))))))

(fn ConstructionScript
  (bind _door1 (Variables|Default|GetDoor1))
  (bind _door2 (Variables|Default|GetDoor2))
  (if (not (Variables|Default|GetClosed))
    (Transformation|SetRelativeLocation _door1 (Variables|Default|GetDoorPosition1) false false)
    (Transformation|SetRelativeScale3D _door1 (Variables|Default|GetDoorScale))
    (Transformation|SetRelativeLocation _door2 (Variables|Default|GetDoorPosition2) false false)
    (Transformation|SetRelativeScale3D _door2 (Variables|Default|GetDoorScale))))