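; Simple elevator actor that shuttles between two placed Path actors each time it is triggered.
; TriggerActivator always starts a move, while actor overlap starts one only when ButtonOnly is off.
; A DoOnce blocks retriggers while MoveComponentTo slides the root to the target over a fixed time, then InitEnd flips to the other end and the gate resets.
; The construction script snaps the actor to the first Path point.
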(event Custom|UP/Down
  (Utilities|FlowControl|DoOnce false :!label _label
    (:Completed
      (Components|MoveComponentTo (Variables|Default|GetDefaultSceneRoot) (Transformation|GetActorLocation (Utilities|Array|Get(acopy) (Variables|Default|GetPath) (Variables|Default|GetInit/End))) "0, 0, 0" false false 2.0 false)
      (Variables|Default|SetInit/End (Math|Integer|%(Integer) (+ (Variables|Default|GetInit/End) 1) 2))
      (goto _label Reset))))

(event Collision|EventActorBeginOverlap
  (params (OtherActor :type Actor%20Object%20Reference))
  (if (not (Variables|Default|GetButtonOnly))
    (CallFunction|UP/Down)))

(event EventTick
  (params (DeltaSeconds :type Float%20%28single-precision%29)))

(event EventTriggerActivator
  (CallFunction|UP/Down))

(fn ConstructionScript
  (Transformation|SetActorLocation (Transformation|GetActorLocation (Utilities|Array|Get(acopy) (Variables|Default|GetPath))) false false)
  (Variables|Default|SetInit/End 1))