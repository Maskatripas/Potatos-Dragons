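; BasicConveyerSwitch is a switch actor that changes the direction of a linked conveyer belt when activated.
; On TriggerActivator it passes the current entry of a list of possible directions to the belt's ChangeConveyerDirection.
; It then advances the index with a modulo wrap, so repeated activations cycle through the directions in order.
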(event EventTriggerActivator
  ;[1 1 1] CallToChangeDirection
  (Default|ChangeConveyerDirection (Variables|Default|GetConveyerBeltChanged) (Utilities|Array|Get(acopy) (Variables|Default|GetPosibleDirections) (Variables|Default|GetCurrentDirection)))
  ;[1 1 1] CalculateNextDirection
  (Variables|Default|SetCurrentDirection (Math|Integer|%(Integer) (+ (Variables|Default|GetCurrentDirection) 1) (Utilities|Array|Length (Variables|Default|GetPosibleDirections)))))

(fn ConstructionScript)