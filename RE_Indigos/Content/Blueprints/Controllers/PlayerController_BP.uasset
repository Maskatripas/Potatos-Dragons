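; Player controller that handles the pause menu input.
; Pressing Pause either pauses the game and creates and displays a PauseMenu_BP widget, or unpauses and removes it, using the stored widget's validity as the toggle state.
; Each menu change happens only if the pause call succeeds.
; An Interact function taking a Telekinesis input is stubbed to return false.
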(event Input|ActionEvents|InputActionPause
  (params (Key :type Key%20Structure))
  ;[1 1 1] Pause Menu Input
  (:Pressed
    (Utilities|IsValid (Variables|Default|GetPauseMenu)
      (:Is%20Valid
        (bind _returnvalue (Game|SetGamePaused false))
        (if _returnvalue
          (Widget|RemovefromParent (Variables|Default|GetPauseMenu))
          (Variables|Default|SetPauseMenu 0)))
      (:Is%20Not%20Valid
        (bind _returnvalue_2 (Game|SetGamePaused true))
        (if _returnvalue_2
          (bind _returnvalue_3 (UserInterface|CreateWidget "/Game/UI/PauseMenu_BP.PauseMenu_BP_C"))
          (bind _output_get (Variables|Default|SetPauseMenu _returnvalue_3))
          (UserInterface|Viewport|AddtoViewport _output_get 0))))))

(fn ConstructionScript)

(fn Interact
  (params (Telekinesis :type Boolean))
  (return false))