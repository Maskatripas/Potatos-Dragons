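; AI controller that makes its controlled MainChar_BP follow the player's pawn, toggled on and off through PlayerController_BP.
; On BeginPlay it binds to the player controller's follow event, which starts or clears a looping timer.
; Each timer tick re-issues an AI Move To toward the player while the character's CanMove flag is set, otherwise it ends following and stops movement.
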(event Custom|Follow%20Toggle
  (if (Utilities|Time|IsTimerActivebyHandle (Variables|Default|GetIsFollowing))
    (Utilities|Time|ClearandInvalidateTimerbyHandle (Variables|Default|GetIsFollowing))
    (AI|Navigation|StopMovement)
    (else
      (bind _returnvalue (Utilities|Time|SetTimerbyEvent (delegate Custom|Follow%20Player) 0.2 true))
      (Variables|Default|SetIsFollowing _returnvalue))))

(event Custom|Follow%20Player
  (bind _asmain_char_bp (Utilities|Casting|CastToMainChar_BP (Pawn|GetControlledPawn)))
  (if (Variables|/Game/Blueprints/Actors/MainChar_BP.MainChar_BP_C|GetCan%20Move _asmain_char_bp)
    (AI|AIMoveTo _asmain_char_bp "0, 0, 0" (Game|Player|GetPlayerPawn 0) 25.0 true)
    (else
      (Utilities|Time|ClearandInvalidateTimerbyHandle (Variables|Default|GetIsFollowing))
      (AI|Navigation|StopMovement))))

(event EventBeginPlay
  (bind _asplayer_controller_bp (Utilities|Casting|CastToPlayerController_BP (Game|GetPlayerController 0)))
  (EventDispatchers|BindEventtoFollowPlayer _asplayer_controller_bp (delegate Custom|Follow%20Toggle)))

(fn ConstructionScript)