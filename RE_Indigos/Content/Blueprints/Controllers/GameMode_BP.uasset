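; Game mode that sets up a two-character pair, Rafi and Sam, when the default pawn spawns for a PlayerController_BP.
; It reuses existing instances or spawns them at offsets from the start transform, then caches references and transforms.
; The PlayerStart tag picks the player's pawn, defaulting to Rafi, and a spawned follower AI controller possesses the other.
; Other controllers get the parent spawn behavior.
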(fn ConstructionScript)

(fn SpawnDefaultPawnfor
  (params (NewPlayer :type Controller%20Object%20Reference) (StartSpot :type Actor%20Object%20Reference))
  (bind _asplayer_start (Utilities|Casting|CastToPlayerStart StartSpot))
  (bind _output_get (Variables|References|SetPlayerStartRef _asplayer_start))
  (bind _returnvalue (|CallParentFunction NewPlayer _output_get))
  (return _returnvalue))

(fn SpawnDefaultPawnatTransform
  (params (NewPlayer :type Controller%20Object%20Reference) (SpawnTransform :type Transform%20%28by%20ref%29))
  (Variables|Default|SetPlayerStartTransform SpawnTransform)
  (bind _asplayer_controller_bp (Utilities|Casting|CastToPlayerController_BP NewPlayer)
    (:then
      (Variables|References|SetPlayerRef _asplayer_controller_bp)
      (Utilities|FlowControl|Sequence
        (:then_0
          (bind _output (Utilities|InitializeCharacters (Variables|Classes|GetRafi%20Class) (Utilities|OffsetSpawn (Variables|Default|GetPlayerStartTransform) -25.0 25.0 -25.0)))
          (bind _asrafi_bp (Utilities|Casting|CastToRafi_BP _output))
          (bind _output_get (Variables|References|SetRafiRef _asrafi_bp))
          (Variables|Default|SetSpawnTransform_Rafi (Transformation|GetActorTransform _output_get)))
        (:then_1
          (bind _output_2 (Utilities|InitializeCharacters (Variables|Classes|GetSam%20Class) (Utilities|OffsetSpawn (Variables|Default|GetPlayerStartTransform) 0.0 -25.0 25.0)))
          (bind _assam_bp (Utilities|Casting|CastToSam_BP _output_2))
          (bind _output_get_2 (Variables|References|SetSamRef _assam_bp))
          (Variables|Default|SetSpawnTransform_Sam (Transformation|GetActorTransform _output_get_2)))
        (:then_2
          (bind (_main_pawn _other_pawn) (Utilities|ChoosePawn (Variables|References|GetPlayerStartRef) (Variables|References|GetRafiRef) (Variables|References|GetSamRef)))
          (bind _returnvalue (Game|SpawnActorfromClass (Variables|Classes|GetFollower%20AI%20Class) (Math|Transform|MakeTransform "0, 0, 0" "0, 0, 0" "1,1,1") "Undefined" 0 0))
          (Pawn|Possess _returnvalue _other_pawn)
          (return _main_pawn))))
    (:CastFailed
      (bind _returnvalue_2 (|CallParentFunction NewPlayer SpawnTransform))
      (return _returnvalue_2))))