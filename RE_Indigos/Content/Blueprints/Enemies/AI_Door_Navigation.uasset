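; AI navigation trigger placed at a door that directs searching enemies through to the other side.
; When an AICharacter overlaps it while searching, it checks that the last player position lies within the controller's acceptance distance.
; It then picks whichever of its two entrance points is farther from the enemy.
; That point is written to the Blackboard as DoorLocation and DoorDetection is set true.
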(event EventBeginPlay)

(event Collision|EventActorBeginOverlap
  (params (OtherActor :type Actor%20Object%20Reference))
  (bind _asaicharacter (Utilities|Casting|CastToAICharacter OtherActor))
  (bind _asaicharacter_controller (Utilities|Casting|CastToAICharacterController (AI|GetAIController _asaicharacter)))
  (if (and (ScalableFloat|GetValueasBool (AI|GetBlackboard _asaicharacter_controller) (Utilities|Name|MakeLiteralName "SearchingForPlayer")) (> (Variables|/Game/Blueprints/Marc/EnemyAI/AICharacterController.AICharacterController_C|GetAcceptanceDoorDistance _asaicharacter_controller) (Math|Vector|VectorLength (- (AI|Components|Blackboard|GetValueasVector (AI|GetBlackboard _asaicharacter_controller) (Utilities|Name|MakeLiteralName "LastPlayerPosition")) (Transformation|GetActorLocation _asaicharacter)))))
    (bind _destinylocation (CallFunction|GetDestinyLocation (Transformation|GetActorLocation _asaicharacter)))
    (AI|Components|Blackboard|SetValueasVector (AI|GetBlackboard _asaicharacter_controller) (Utilities|Name|MakeLiteralName "DoorLocation") _destinylocation)
    (AI|Components|Blackboard|SetValueasBool (AI|GetBlackboard _asaicharacter_controller) (Utilities|Name|MakeLiteralName "DoorDetection") true)))

(fn ConstructionScript)

(fn GetDestinyLocation
  (params (EnemyLocation :type Vector))
  (bind _entrance1 (Variables|Default|GetEntrance1))
  (bind _entrance2 (Variables|Default|GetEntrance2))
  (bind _returnvalue (Transformation|GetWorldLocation _entrance2))
  (bind _returnvalue_2 (Transformation|GetWorldLocation _entrance1))
  (if (< (Math|Vector|VectorLength (- _returnvalue_2 EnemyLocation)) (Math|Vector|VectorLength (- _returnvalue EnemyLocation)))
    (return _returnvalue)
    (else
      (return _returnvalue_2))))