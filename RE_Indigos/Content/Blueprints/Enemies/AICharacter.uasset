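; AICharacter is an enemy character Blueprint with an optional head-mounted green light and a searching look-around animation.
; When LightOn is set, the construction script attaches a child actor to the GL_Head socket and caches it as GreenLight_BP.
; LightEffect swaps a mesh material between green-light and joint looks.
; LookAroundAnimation applies the EnemySearching timeline's yaw relative to the starting rotation, and CleanAnimation stops it.
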(event Custom|LookAroundAnimation
  ;[1 1 1] Animation to look around
  (Variables|Default|SetBaseLookAroundRotation (Transformation|GetActorRotation))
  (bind _enemyrot (Timeline|EnemySearching PlayFromStart)
    (:Update
      (Transformation|SetActorRotation (Math|Rotator|CombineRotators (Math|Rotator|MakeRotator 0.0 0.0 _enemyrot) (Variables|Default|GetBaseLookAroundRotation))))))

(event Custom|CleanAnimation
  ;[1 1 1] Animation to look around
  (bind _enemyrot (Timeline|EnemySearching Stop)
    (:Update
      (Transformation|SetActorRotation (Math|Rotator|CombineRotators (Math|Rotator|MakeRotator 0.0 0.0 _enemyrot) (Variables|Default|GetBaseLookAroundRotation))))))

(event Custom|LightEffect
  (params (Active :type Boolean))
  (bind _mesh (Variables|Character|GetMesh))
  (if Active
    (Rendering|Material|SetMaterial _mesh 1 (Variables|Default|GetGreenLightMaterial))
    (else
      (Rendering|Material|SetMaterial _mesh 1 (Variables|Default|GetJointsMaterial)))))

(fn ConstructionScript
  (if (Variables|Default|GetLight%20On)
    (bind _returnvalue (AddComponent|AddChildActorComponent true))
    (bind _output_get (Variables|Default|SetGreenLightChild _returnvalue))
    (Transformation|AttachComponentToComponent _output_get (Variables|Character|GetMesh) "GL_Head" "KeepWorld" "KeepWorld" "KeepWorld" true)
    (Transformation|SetRelativeTransform (Variables|Default|GetGreenLightChild) (Math|Transform|MakeTransform "0.000000,0.000000,5.000000" "0.000000,0.000000,-170.000000" "1.000000,1,1") false true)
    (bind _asgreen_light_bp (Utilities|Casting|CastToGreenLight_BP (Variables|/Script/Engine.ChildActorComponent|GetChildActor (Variables|Default|GetGreenLightChild))))
    (Variables|Default|SetGreenLight _asgreen_light_bp)))