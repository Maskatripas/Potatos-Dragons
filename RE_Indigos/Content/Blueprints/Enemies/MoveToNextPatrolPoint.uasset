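; Behavior tree task that picks the next patrol destination for an AICharacter enemy.
; It reads the patrol index from the blackboard and writes that patrol point actor's location to the move location key, without issuing the move itself.
; It then advances the index, wrapping with modulo to loop the route, and finishes successfully.
; A failed cast to AICharacter stops execution without finishing the task.
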(event EventReceiveExecute
  (params (OwnerActor :type Actor%20Object%20Reference))
  (bind _nextpatrolpoint (Variables|Default|GetNextPatrolPoint))
  (bind _returnvalue (Class|BTFunctionLibrary|GetBlackboardValueasInt _nextpatrolpoint))
  ;[1 1 1] We Obtain the current AICharacter
  (bind _asaicharacter (Utilities|Casting|CastToAICharacter (Pawn|GetControlledPawn (AI|GetAIController OwnerActor))))
  ;[1 1 1] We set the value of our new destination
  (AI|BehaviorTree|SetBlackboardValueasVector (Variables|Default|GetMoveLocationKey) (Transformation|GetActorLocation (Utilities|Array|Get(acopy) (Variables|/Game/Blueprints/Enemies/AICharacter.AICharacter_C|GetPatrolPoints _asaicharacter) _returnvalue)))
  ;[1 1 1] We set the value of our new patrol point
  (Class|BTFunctionLibrary|SetBlackboardValueasInt _nextpatrolpoint (Math|Integer|%(Integer) (+ _returnvalue 1) (Utilities|Array|Length (Variables|/Game/Blueprints/Enemies/AICharacter.AICharacter_C|GetPatrolPoints _asaicharacter))))
  (AI|BehaviorTree|FinishExecute true))