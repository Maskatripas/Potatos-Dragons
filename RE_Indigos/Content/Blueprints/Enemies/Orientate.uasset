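; Behavior tree task that orients an enemy AICharacter that has only a single patrol point.
; It gets the controlled pawn from the owner's AI controller, casts it to AICharacter and checks its PatrolPoints array.
; When the second patrol point is not valid, the character's rotation snaps to that of the first point before the task finishes successfully.
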(event EventReceiveExecute
  (params (OwnerActor :type Actor%20Object%20Reference))
  ;[1 1 1] We Obtain the current AICharacter
  (bind _asaicharacter (Utilities|Casting|CastToAICharacter (Pawn|GetControlledPawn (AI|GetAIController OwnerActor)))
    (:then
      ;[1 1 1] If we only have one patrol point we orientate ourselves
      (if (> (Utilities|Array|Length (Variables|/Game/Blueprints/Enemies/AICharacter.AICharacter_C|GetPatrolPoints _asaicharacter)) 0)
        (Utilities|IsValid (Utilities|Array|Get(acopy) (Variables|/Game/Blueprints/Enemies/AICharacter.AICharacter_C|GetPatrolPoints _asaicharacter) 1)
          (:Is%20Valid
            _)
          (:Is%20Not%20Valid
            (Transformation|SetActorRotation _asaicharacter (Transformation|GetActorRotation (Utilities|Array|Get(acopy) (Variables|/Game/Blueprints/Enemies/AICharacter.AICharacter_C|GetPatrolPoints _asaicharacter))))))))
    (:CastFailed
      _))
  (AI|BehaviorTree|FinishExecute true))