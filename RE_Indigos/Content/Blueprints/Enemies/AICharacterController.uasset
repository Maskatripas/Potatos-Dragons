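; AI controller for AICharacter enemies that runs their behavior tree and feeds it perception of the player.
; On possess it starts AI_BT and resets the patrol index and door-detection blackboard keys.
; Perception updates on player-tagged actors set the can-see, searching and last-known-position keys, switching to searching when sight is lost, then call CleanAnimation on the character.
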(event OnTargetPerceptionUpdated(AIPerception)
  (params (Actor :type Actor%20Object%20Reference) (Stimulus :type AI%20Stimulus%20Structure))
  (bind _bsuccessfullysensed (Utilities|Struct|BreakAIStimulus Stimulus))
  (bind _returnvalue (Utilities|Name|MakeLiteralName "SearchingForPlayer"))
  ;[1 1 1] AISightSense_ChangedValue
  (if (Actor|ActorHasTag Actor (Variables|Default|GetPlayerTag))
    ;[1 1 1] SetCanSeePlayerKey
    (AI|Components|Blackboard|SetValueasBool (AI|GetBlackboard 0) (Utilities|Name|MakeLiteralName "CanSeePlayer") _bsuccessfullysensed)
    ;[1 1 1] SetSearchingForPlayerKey
    (if _bsuccessfullysensed
      (AI|Components|Blackboard|SetValueasBool (AI|GetBlackboard 0) _returnvalue false)
      (else
        (AI|Components|Blackboard|SetValueasBool (AI|GetBlackboard 0) _returnvalue true)))
    ;[1 1 1] SetLastPlayerPositionValue
    (AI|Components|Blackboard|SetValueasVector (AI|GetBlackboard 0) (Utilities|Name|MakeLiteralName "LastPlayerPosition") (Transformation|GetActorLocation Actor))
    (bind _asaicharacter (Utilities|Casting|CastToAICharacter (Pawn|GetControlledPawn)))
    (Default|CleanAnimation _asaicharacter)))

(event EventOnPossess
  (params (PossessedPawn :type Pawn%20Object%20Reference))
  (bind _returnvalue (AI|GetBlackboard 0))
  ;[1 1 1] RunBehaviourTree
  (Utilities|Casting|CastToAICharacter PossessedPawn)
  (AI|RunBehaviorTree "/Game/Blueprints/Enemies/AI_BT.AI_BT")
  ;[1 1 1] SetDefaultPatrolIndexValue
  (Class|BlackboardComponent|SetValueasInt _returnvalue (Utilities|Name|MakeLiteralName "NextPatrolPoint"))
  (AI|Components|Blackboard|SetValueasBool _returnvalue (Utilities|Name|MakeLiteralName "DoorDetection") false))

(event EventTick
  (params (DeltaSeconds :type Float%20%28single-precision%29)))

(fn ConstructionScript)