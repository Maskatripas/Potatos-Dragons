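; Rafi is a playable character with telekinesis over tagged objects and activators, and can hand control to Sam.
; Holding a power input locks movement and box-traces visible Telekinesis-interface actors, ranked by angle, distance and height, with debug shapes highlighting the selection.
; The right axis cycles candidates during the hold, and release starts telekinesis on the target.
; Interface messages then move, rotate or activate it until cancel or another press ends control.
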(event EventPowerUp
  (params (Axis%20Value :type Float%20%28single-precision%29))
  ;[1 1 1] Power Motion Input
  (if (Variables|Default|GetActive%20Power)
    (if (not (Audio|Components|Audio|IsPlaying (Variables|Default|GetTelekinesis%20Display)))
      (Class|TelekinesisInterfaceBP|TelekinesisUp(Message) (Variables|Default|GetPowerTarget) self Axis%20Value (Variables|Default|GetPowerRangeHeight)))))

(event EventPowerRight
  (params (Axis%20Value :type Float%20%28single-precision%29))
  ;[1 1 1] Power Motion Input
  (if (Variables|Default|GetActive%20Power)
    (if (or (Audio|Components|Audio|IsPlaying (Variables|Default|GetTelekinesis%20Display)) (Audio|Components|Audio|IsPlaying (Variables|Default|GetTelekinesis%20Activator%20Display)))
      (bind _item (Utilities|Traverse Axis%20Value (Variables|Default|GetPowerArray))
        (:Result
          (Variables|Default|SetPowerTarget (Components|GetOwner _item))))
      (else
        (Class|TelekinesisInterfaceBP|TelekinesisRight(Message) (Variables|Default|GetPowerTarget) self Axis%20Value (Variables|Default|GetPowerRange))))))

(event EventTelekinesisCancel
  ;[1 1 1] Telekinesis Input
  (Variables|Default|GetPowerTarget
    (:then
      (Utilities|FlowControl|Sequence
        (:then_0
          (Class|TelekinesisInterfaceBP|TelekinesisEnd(Message) (Variables|Default|GetPowerTarget))
          (Variables|Default|SetPowerTarget 0)
          (Utilities|Array|Clear (Variables|Default|GetPowerArray)))
        (:then_1
          (Class|AnimInterfaceBP|TelekinesisAnim(Message) (Components|SkeletalMesh|GetAnimInstance (Variables|Character|GetMesh)) 1)
          (Variables|Default|SetActive%20Power false)
          (Variables|Default|SetCan%20Move true))))
    (:else)))

(event EventSubPowerPressed
  (Variables|Default|GetPowerTarget
    (:then
      (Utilities|FlowControl|Sequence
        (:then_0
          (Class|TelekinesisInterfaceBP|TelekinesisEnd(Message) (Variables|Default|GetPowerTarget))
          (Variables|Default|SetPowerTarget 0)
          (Utilities|Array|Clear (Variables|Default|GetPowerArray)))
        (:then_1
          (Class|AnimInterfaceBP|TelekinesisAnim(Message) (Components|SkeletalMesh|GetAnimInstance (Variables|Character|GetMesh)) 1)
          (Variables|Default|SetActive%20Power false)
          (Variables|Default|SetCan%20Move true))))
    (:else
      (Utilities|FlowControl|DoOnce false
        (:Completed
          (Utilities|FlowControl|Sequence
            (:then_0
              (Variables|Default|SetActive%20Power true)
              (Variables|Default|SetCan%20Move false)
              (Utilities|FlowControl|Sequence
                (:then_0
                  (Class|AnimInterfaceBP|TelekinesisAnim(Message) (Components|SkeletalMesh|GetAnimInstance (Variables|Character|GetMesh))))
                (:then_1
                  (bind (_result _sorted_array) (CallFunction|SortTelekinesis (Transformation|GetWorldLocation (Variables|Character|GetMesh)) (Variables|Default|GetActivatorTag)))
                  (if _result
                    (bind _output_get (Variables|Default|SetPowerArray _sorted_array))
                    (Variables|Default|SetPowerTarget (Components|GetOwner (Utilities|Array|Get(acopy) _output_get)))))))
            (:then_1
              (Timeline|Telekinesis%20Activator%20Display Play
                (:Update
                  (Rendering|Debug|DrawDebugCircle (Transformation|GetWorldLocation (Variables|Character|GetMesh)) (Variables|Default|GetPowerRadius) 50 "(R=0.500000,G=0.000000,B=1.000000,A=1.000000)" 0.0 5.0 "1.000000,0.000000,0.000000" "0.000000,1.000000,0.000000")
                  (for _array_element (Variables|Default|GetPowerArray)
                    (bind _asbox_collision (Utilities|Casting|CastToBoxComponent _array_element))
                    (if (== (Components|GetOwner _array_element) (Variables|Default|GetPowerTarget))
                      (Rendering|Debug|DrawDebugBox (Transformation|GetWorldLocation _array_element) (Components|Box|GetScaledBoxExtent _asbox_collision) "(R=1.000000,G=0.000000,B=0.000000,A=1.000000)" (Transformation|GetWorldRotation _array_element) 0.0 5.0)
                      (else
                        (Rendering|Debug|DrawDebugBox (Transformation|GetWorldLocation _array_element) (Components|Box|GetScaledBoxExtent _asbox_collision) "(R=0.500000,G=0.000000,B=1.000000,A=1.000000)" (Transformation|GetWorldRotation _array_element) 0.0 5.0)))))))))))))

(event EventSubPowerReleased
  (Utilities|FlowControl|Sequence
    (:then_0
      (Utilities|FlowControl|DoOnce false) ; enters at Reset
    )
    (:then_1
      (Timeline|Telekinesis%20Activator%20Display Stop
        (:Update
          (Rendering|Debug|DrawDebugCircle (Transformation|GetWorldLocation (Variables|Character|GetMesh)) (Variables|Default|GetPowerRadius) 50 "(R=0.500000,G=0.000000,B=1.000000,A=1.000000)" 0.0 5.0 "1.000000,0.000000,0.000000" "0.000000,1.000000,0.000000")
          (for _array_element (Variables|Default|GetPowerArray)
            (bind _asbox_collision (Utilities|Casting|CastToBoxComponent _array_element))
            (if (== (Components|GetOwner _array_element) (Variables|Default|GetPowerTarget))
              (Rendering|Debug|DrawDebugBox (Transformation|GetWorldLocation _array_element) (Components|Box|GetScaledBoxExtent _asbox_collision) "(R=1.000000,G=0.000000,B=0.000000,A=1.000000)" (Transformation|GetWorldRotation _array_element) 0.0 5.0)
              (else
                (Rendering|Debug|DrawDebugBox (Transformation|GetWorldLocation _array_element) (Components|Box|GetScaledBoxExtent _asbox_collision) "(R=0.500000,G=0.000000,B=1.000000,A=1.000000)" (Transformation|GetWorldRotation _array_element) 0.0 5.0)))))))
    (:then_2
      (bind _powertarget (Variables|Default|GetPowerTarget)
        (:then
          (Class|TelekinesisInterfaceBP|TelekinesisBegin(Message) _powertarget self))
        (:else
          (Utilities|FlowControl|Sequence
            (:then_0
              (Class|AnimInterfaceBP|TelekinesisAnim(Message) (Components|SkeletalMesh|GetAnimInstance (Variables|Character|GetMesh)) 1))
            (:then_1
              (Variables|Default|SetActive%20Power false)
              (Variables|Default|SetCan%20Move true))))))))

(event EventPowerRotateForward
  (params (Axis%20Value :type Float%20%28single-precision%29))
  ;[1 1 1] Power Motion Input
  (if (Variables|Default|GetActive%20Power)
    (if (not (Audio|Components|Audio|IsPlaying (Variables|Default|GetTelekinesis%20Display)))
      (Class|TelekinesisInterfaceBP|TelekinesisRotatePosition(Message) (Variables|Default|GetPowerTarget) self Axis%20Value))))

(event EventPowerRotateRight
  (params (Axis%20Value :type Float%20%28single-precision%29))
  ;[1 1 1] Power Motion Input
  (if (Variables|Default|GetActive%20Power)
    (if (not (Audio|Components|Audio|IsPlaying (Variables|Default|GetTelekinesis%20Display)))
      (Class|TelekinesisInterfaceBP|TelekinesisRotateOrientation(Message) (Variables|Default|GetPowerTarget) self Axis%20Value))))

(event EventMainPowerReleased
  ;[1 1 1] Telekinesis Input
  (Utilities|FlowControl|Sequence
    (:then_0
      (Utilities|FlowControl|DoOnce false) ; enters at Reset
    )
    (:then_1
      (Timeline|Telekinesis%20Display Stop
        (:Update
          (Rendering|Debug|DrawDebugCircle (Transformation|GetWorldLocation (Variables|Character|GetMesh)) (Variables|Default|GetPowerRadius) 50 "(R=0.500000,G=0.000000,B=1.000000,A=1.000000)" 0.0 5.0 "1.000000,0.000000,0.000000" "0.000000,1.000000,0.000000")
          (for _array_element (Variables|Default|GetPowerArray)
            (bind _asbox_collision (Utilities|Casting|CastToBoxComponent _array_element))
            (if (== (Components|GetOwner _array_element) (Variables|Default|GetPowerTarget))
              (Rendering|Debug|DrawDebugBox (Transformation|GetWorldLocation _array_element) (Components|Box|GetScaledBoxExtent _asbox_collision) "(R=1.000000,G=0.000000,B=0.000000,A=1.000000)" (Transformation|GetWorldRotation _array_element) 0.0 5.0)
              (else
                (Rendering|Debug|DrawDebugBox (Transformation|GetWorldLocation _array_element) (Components|Box|GetScaledBoxExtent _asbox_collision) "(R=0.500000,G=0.000000,B=1.000000,A=1.000000)" (Transformation|GetWorldRotation _array_element) 0.0 5.0)))))))
    (:then_2
      (bind _powertarget (Variables|Default|GetPowerTarget)
        (:then
          (Class|TelekinesisInterfaceBP|TelekinesisBegin(Message) _powertarget self))
        (:else
          (Utilities|FlowControl|Sequence
            (:then_0
              (Class|AnimInterfaceBP|TelekinesisAnim(Message) (Components|SkeletalMesh|GetAnimInstance (Variables|Character|GetMesh)) 1))
            (:then_1
              (Variables|Default|SetActive%20Power false)
              (Variables|Default|SetCan%20Move true))))))))

(event EventMainPowerPressed
  ;[1 1 1] Telekinesis Input
  (Variables|Default|GetPowerTarget
    (:then
      (Utilities|FlowControl|Sequence
        (:then_0
          (Class|TelekinesisInterfaceBP|TelekinesisEnd(Message) (Variables|Default|GetPowerTarget))
          (Variables|Default|SetPowerTarget 0)
          (Utilities|Array|Clear (Variables|Default|GetPowerArray)))
        (:then_1
          (Class|AnimInterfaceBP|TelekinesisAnim(Message) (Components|SkeletalMesh|GetAnimInstance (Variables|Character|GetMesh)) 1)
          (Variables|Default|SetActive%20Power false)
          (Variables|Default|SetCan%20Move true))))
    (:else
      (Utilities|FlowControl|DoOnce false
        (:Completed
          (Utilities|FlowControl|Sequence
            (:then_0
              (Variables|Default|SetActive%20Power true)
              (Variables|Default|SetCan%20Move false)
              (Utilities|FlowControl|Sequence
                (:then_0
                  (Class|AnimInterfaceBP|TelekinesisAnim(Message) (Components|SkeletalMesh|GetAnimInstance (Variables|Character|GetMesh))))
                (:then_1
                  (bind (_result _sorted_array) (CallFunction|SortTelekinesis (Transformation|GetWorldLocation (Variables|Character|GetMesh)) (Variables|Default|GetObjectTag)))
                  (if _result
                    (bind _output_get (Variables|Default|SetPowerArray _sorted_array))
                    (Variables|Default|SetPowerTarget (Components|GetOwner (Utilities|Array|Get(acopy) _output_get)))))))
            (:then_1
              (Timeline|Telekinesis%20Display Play
                (:Update
                  (Rendering|Debug|DrawDebugCircle (Transformation|GetWorldLocation (Variables|Character|GetMesh)) (Variables|Default|GetPowerRadius) 50 "(R=0.500000,G=0.000000,B=1.000000,A=1.000000)" 0.0 5.0 "1.000000,0.000000,0.000000" "0.000000,1.000000,0.000000")
                  (for _array_element (Variables|Default|GetPowerArray)
                    (bind _asbox_collision (Utilities|Casting|CastToBoxComponent _array_element))
                    (if (== (Components|GetOwner _array_element) (Variables|Default|GetPowerTarget))
                      (Rendering|Debug|DrawDebugBox (Transformation|GetWorldLocation _array_element) (Components|Box|GetScaledBoxExtent _asbox_collision) "(R=1.000000,G=0.000000,B=0.000000,A=1.000000)" (Transformation|GetWorldRotation _array_element) 0.0 5.0)
                      (else
                        (Rendering|Debug|DrawDebugBox (Transformation|GetWorldLocation _array_element) (Components|Box|GetScaledBoxExtent _asbox_collision) "(R=0.500000,G=0.000000,B=1.000000,A=1.000000)" (Transformation|GetWorldRotation _array_element) 0.0 5.0)))))))))))))

(event EventInputInteraction
  (bind _powertarget (Variables|Default|GetPowerTarget)
    (:then
      (Class|TelekinesisInterfaceBP|TelekinesisActivator(Message) _powertarget))
    (:else)))

(event EventPowerForward
  (params (Axis%20Value :type Float%20%28single-precision%29))
  ;[1 1 1] Power Motion Input
  (if (Variables|Default|GetActive%20Power)
    (if (not (Audio|Components|Audio|IsPlaying (Variables|Default|GetTelekinesis%20Display)))
      (Class|TelekinesisInterfaceBP|TelekinesisForward(Message) (Variables|Default|GetPowerTarget) self Axis%20Value (Variables|Default|GetPowerRange)))))

(event Input|ActionEvents|InputActionSam
  (params (Key :type Key%20Structure))
  ;[1 1 1] Switch to Sam
  (:Pressed
    (bind _asgame_mode_bp (Utilities|Casting|CastToGameMode_BP (Game|GetGameMode)))
    (CallFunction|SwitchCharacter (Variables|/Game/Blueprints/Controllers/GameMode_BP.GameMode_BP_C|GetSamRef _asgame_mode_bp) (Pawn|GetControlRotation :!class /Script/Engine.Pawn))))

(fn ConstructionScript)

(fn SortTelekinesis
  (params (Center :type Vector) (Tag :type Name))
  (bind _sortingloop (LocalVariables|GetSortingLoop))
  (bind _powerradius (Variables|Default|GetPowerRadius))
  (bind _capsulecomponent (Variables|Default|GetCapsuleComponent))
  (bind _returnvalue (Transformation|GetWorldLocation _capsulecomponent))
  (bind _returnvalue_2 (Class|CapsuleComponent|GetScaledCapsuleHalfHeightWithoutHemisphere _capsulecomponent))
  (bind _returnvalue_3 (- (.z _returnvalue) _returnvalue_2))
  (bind _returnvalue_4 (- _returnvalue_3 5.0))
  (bind _outhits (Class|KismetSystemLibrary|BoxTraceMultiforObjects Center Center (Math|Vector|MakeVector _powerradius _powerradius (Variables|Default|GetPowerRadiusHeight)) "0, 0, 0" (Utilities|Array|MakeArray "ObjectTypeQuery2") false 0 "None" true))
  (for _array_element _outhits
    (LocalVariables|SetLoopAngle (.Angle (Utilities|GetSortingParameters (.hitcomponent _array_element))))
    (bind _output_get (LocalVariables|SetLoopDistance (.Distance (Utilities|GetSortingParameters (.hitcomponent _array_element)))))
    (LocalVariables|SetLoopHeight (.Height (Utilities|GetSortingParameters (.hitcomponent _array_element))))
    (if (Math|Boolean|ANDBoolean (<= _output_get (Variables|Default|GetPowerRadius)) (Utilities|DoesObjectImplementInterface (.hitactor _array_element) "/Game/Blueprints/Libraries/Interfaces/Telekinesis_Interface_BP.Telekinesis_Interface_BP_C") (Actor|ActorHasTag (.hitactor _array_element) Tag))
      (bind (_outhit _returnvalue_5) (Collision|LineTraceByChannel (Transformation|GetActorLocation) (Transformation|GetActorLocation (.hitactor _array_element)) "TraceTypeQuery1" false 0 "None"))
      (if (or (not _returnvalue_5) (== (.hitactor _outhit) (.hitactor _array_element)))
        (bind _outhit_2 (Class|KismetSystemLibrary|SphereTraceSinglebyProfile (Math|Vector|MakeVector (.x _returnvalue) (.y _returnvalue) _returnvalue_4) (Math|Vector|MakeVector (.x _returnvalue) (.y _returnvalue) _returnvalue_4) (- (Components|Capsule|GetScaledCapsuleRadius _capsulecomponent) 1.0) (Collision|GetCollisionProfileName _capsulecomponent) false 0 "None" true))
        (if (!= (.hitactor _outhit_2) (.hitactor _array_element))
          (bind _output_get_2 (LocalVariables|SetLoopComponent (.hitcomponent _array_element)))
          (Utilities|Array|Add _sortingloop _output_get_2)
          (bind _arrayindex (Utilities|Array|ReverseforEachLoop _sortingloop)
            (:LoopBody
              (switch int _arrayindex
                (:Default
                  (Math|Float|CompareFloat (.Angle (Utilities|GetSortingParameters (Utilities|Array|Get(acopy) _sortingloop (- _arrayindex 1)))) (LocalVariables|GetLoopAngle) ; First priority: Objects that are closest\nto Rafi's straight line of sight.
                    (:==
                      (Math|Float|CompareFloat (.Distance (Utilities|GetSortingParameters (Utilities|Array|Get(acopy) _sortingloop (- _arrayindex 1)))) (LocalVariables|GetLoopDistance) ; Second priority: Objects that are \nclosest to Rafi.
                        (:==
                          (Math|Float|CompareFloat (.Height (Utilities|GetSortingParameters (Utilities|Array|Get(acopy) _sortingloop (- _arrayindex 1)))) (LocalVariables|GetLoopHeight) ; Third priority: Objects that are\nat the lowest height.
                            (:<
                              _)))
                        (:<
                          _)))
                    (:<
                      _))
                  (Utilities|Array|Swap (LocalVariables|GetSortingLoop) (- _arrayindex 1) _arrayindex)))))))))
  (return (Utilities|IsValid (LocalVariables|GetLoopComponent)) (LocalVariables|GetSortingLoop)))

(fn TelekinesisPileUp
  (return 0))