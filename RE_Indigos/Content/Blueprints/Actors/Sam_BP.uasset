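; Sam is a playable character who throws a Rubik cube projectile, then teleports to it or erases it, and can swap to Rafi.
; While main power is held, a timeline redraws a debug-line predicted path as input turns Sam and adjusts distance and arc.
; Release triggers a throw animation, whose notify spawns the cube and launches it with a suggested custom-arc velocity.
; Animation notifies also toggle cube visibility and restore movement.
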(event EventThrowAnim
  (params (Notify :type Integer))
  (bind _launch_velocity (Variables|Default|GetLaunch%20Velocity))
  (bind _mesh (Variables|Character|GetMesh))
  (bind _returnvalue (Transformation|GetSocketLocation _mesh "CubeSocket"))
  ;[1 1 1] Rubik Cube Throw Input
  (switch int Notify
    (:0
      (Rendering|SetVisibility (Variables|Default|GetRubikCube) false false)
      (bind _launch_target (Utilities|GetThrowParameters _returnvalue))
      (bind _returnvalue_2 (Game|SpawnActorfromClass "/Game/Blueprints/Objects/CubeProjectile_BP.CubeProjectile_BP_C" (Math|Transform|MakeTransform _returnvalue (Math|Rotator|FindLookatRotation _returnvalue _launch_target) "1,1,1") "AlwaysSpawn" 0 self))
      (bind _output_get (Variables|Default|SetCubeProjectile _returnvalue_2))
      (Collision|IgnoreActorwhenMoving (Variables|/Game/Blueprints/Objects/MoveableObject_BP.MoveableObject_BP_C|GetBoxComponent _output_get) self true)
      (Collision|IgnoreActorwhenMoving (Variables|Default|GetCapsuleComponent) _output_get true)
      (Physics|AddImpulse (Variables|/Game/Blueprints/Objects/MoveableObject_BP.MoveableObject_BP_C|GetBoxComponent _output_get) _launch_velocity "None" true)
      (Class|PrimitiveComponent|AddAngularImpulseinDegrees (Variables|/Game/Blueprints/Objects/MoveableObject_BP.MoveableObject_BP_C|GetBoxComponent _output_get) (* (Math|Vector|GetRightVector (Math|Rotator|FindLookatRotation _returnvalue _launch_target)) (Math|Vector|VectorLength _launch_velocity)) "None" true))
    (:1
      (Utilities|FlowControl|Sequence
        (:then_0
          (Utilities|FlowControl|DoOnce false) ; enters at Reset
        )
        (:then_1
          (Variables|Default|SetCan%20Move true))))))

(event EventDestroyAnim
  (params (Notify :type Integer))
  (bind _rubikcube (Variables|Default|GetRubikCube))
  ;[1 1 1] Rubik Cube Throw Input
  (switch int Notify
    (:0
      (Rendering|SetVisibility _rubikcube true false)
      (Actor|DestroyActor (Variables|Default|GetCubeProjectile)))
    (:1
      (Rendering|SetVisibility _rubikcube false false))
    (:2
      (Variables|Default|SetErasing false)
      (Variables|Default|SetCan%20Move true)
      (Variables|Default|SetActive%20Power false))))

(event EventMainPowerPressed
  (bind _cubespawner (Variables|Default|GetCubeSpawner))
  (bind _returnvalue (Transformation|GetWorldLocation _cubespawner))
  ;[1 1 1] Rubik Cube Throw Input
  (if (not (Variables|Default|GetErasing))
    (bind _cubeprojectile (Variables|Default|GetCubeProjectile)
      (:then
        (if (Variables|/Game/Blueprints/Objects/CubeProjectile_BP.CubeProjectile_BP_C|GetReleased _cubeprojectile)
          (Variables|Default|SetErasing true)
          (Variables|Default|SetCan%20Move false)
          (Class|AnimInterfaceBP|DestroyAnim(Message) (Components|SkeletalMesh|GetAnimInstance (Variables|Character|GetMesh)))))
      (:else
        (Utilities|FlowControl|DoOnce false
          (:Completed
            (Utilities|FlowControl|Sequence
              (:then_0
                (Variables|Default|SetActive%20Power true)
                (Variables|Default|SetCan%20Move false)
                (Variables|ArcParameters|SetThrow%20Offset (Variables|ArcParameters|GetThrow%20Offset%20Min))
                (Variables|ArcParameters|SetThrow%20Arc (Variables|ArcParameters|GetThrow%20Arc%20Max)))
              (:then_1
                (Timeline|Main%20Power Play
                  (:Update
                    (bind _launch_velocity (Utilities|GetThrowParameters _returnvalue))
                    (bind (_outhit _outpathpositions) (Class|GameplayStatics|BlueprintPredictProjectilePathbyTraceChannel _returnvalue _launch_velocity true 0.0 "ECC_Visibility" false (Utilities|Array|MakeArray self) "None" 0.0 15.0 5.0))
                    (|DrawDebugTrajectory _outpathpositions (.location _outhit))))))))))))

(event EventMainPowerReleased
  (bind _cubespawner (Variables|Default|GetCubeSpawner))
  (bind _returnvalue (Transformation|GetWorldLocation _cubespawner))
  ;[1 1 1] Rubik Cube Throw Input
  (if (not (Variables|Default|GetErasing))
    (Variables|Default|GetCubeProjectile
      (:then)
      (:else
        (Utilities|FlowControl|Sequence
          (:then_0
            (Utilities|FlowControl|DoOnce false) ; enters at Reset
          )
          (:then_1
            (Timeline|Main%20Power Stop
              (:Update
                (bind _launch_velocity (Utilities|GetThrowParameters _returnvalue))
                (bind (_outhit _outpathpositions) (Class|GameplayStatics|BlueprintPredictProjectilePathbyTraceChannel _returnvalue _launch_velocity true 0.0 "ECC_Visibility" false (Utilities|Array|MakeArray self) "None" 0.0 15.0 5.0))
                (|DrawDebugTrajectory _outpathpositions (.location _outhit)))))
          (:then_2
            (Utilities|FlowControl|DoOnce false
              (:Completed
                (Rendering|SetVisibility (Variables|Default|GetRubikCube) true false)
                (Class|AnimInterfaceBP|ThrowAnim(Message) (Components|SkeletalMesh|GetAnimInstance (Variables|Character|GetMesh)))))))))))

(event EventPowerForward
  (params (Axis%20Value :type Float%20%28single-precision%29))
  (bind _throw_offset_max (Variables|ArcParameters|GetThrow%20Offset%20Max))
  (bind _throw_offset_min (Variables|ArcParameters|GetThrow%20Offset%20Min))
  ;[1 1 1] Cube Throw Distance Input
  (if (Audio|Components|Audio|IsPlaying (Variables|Default|GetMain%20Power))
    (bind _output_get (Variables|ArcParameters|SetThrow%20Offset (|CalcThrowOffset Axis%20Value 5.0 (Variables|ArcParameters|GetThrow%20Offset) _throw_offset_min _throw_offset_max)))
    (Variables|ArcParameters|SetThrow%20Arc (Math|Float|MapRangeClamped _output_get _throw_offset_min _throw_offset_max (Variables|ArcParameters|GetThrow%20Arc%20Min) (Variables|ArcParameters|GetThrow%20Arc%20Max)))))

(event EventPowerRight
  (params (Axis%20Value :type Float%20%28single-precision%29))
  ;[1 1 1] Cube Throw Distance Input
  (if (Audio|Components|Audio|IsPlaying (Variables|Default|GetMain%20Power))
    (Class|Actor|AddActorWorldRotation (Math|Rotator|MakeRotator 0.0 0.0 (* Axis%20Value 2.0)))))

(event EventSubPowerPressed
  ;[1 1 1] Teleport
  (bind _cubeprojectile (Variables|Default|GetCubeProjectile)
    (:then
      (bind _teleportpoint (Variables|/Game/Blueprints/Objects/CubeProjectile_BP.CubeProjectile_BP_C|GetTeleportPoint _cubeprojectile)
        (:then
          (Variables|Default|SetCan%20Move false)
          (Class|AnimInterfaceBP|TeleportAnim(Message) (Components|SkeletalMesh|GetAnimInstance (Variables|Character|GetMesh)))
          (Transformation|Teleport (Transformation|GetWorldLocation (Variables|/Game/Blueprints/Objects/TeleportTarget_BP.TeleportTarget_BP_C|GetTeleportCollider _teleportpoint)) (Transformation|GetActorRotation))
          (Actor|DestroyActor (Variables|Default|GetCubeProjectile)))
        (:else)))
    (:else)))

(event EventTeleportAnim
  (params (Notify :type Integer))
  ;[1 1 1] Teleport
  (switch int Notify
    (:0
      (Variables|Default|SetCan%20Move true)
      (Variables|Default|SetActive%20Power false))))

(event Input|ActionEvents|InputActionRafi
  (params (Key :type Key%20Structure))
  ;[1 1 1] Switch to Rafi
  (:Pressed
    (bind _asgame_mode_bp (Utilities|Casting|CastToGameMode_BP (Game|GetGameMode)))
    (CallFunction|SwitchCharacter (Variables|/Game/Blueprints/Controllers/GameMode_BP.GameMode_BP_C|GetRafiRef _asgame_mode_bp) (Pawn|GetControlRotation :!class /Script/Engine.Pawn))))

(fn ConstructionScript)