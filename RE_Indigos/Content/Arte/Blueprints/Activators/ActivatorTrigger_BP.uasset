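; ActivatorTrigger_BP is an interactable trigger that sends its Channel to a list of Activables when used directly or, if enabled, by telekinesis.
; In Hold mode, each activation flips Holding and swaps a mesh material to show the state.
; The construction script enables telekinesis query collision only when that option is on.
; Retriggerable delays auto-hide the interaction widget and the custom-depth stencil highlight shown during telekinesis targeting.
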(event Custom|Event%20Activate
  ;[1 1 1] Interface Events
  (if (Variables|Default|GetHold)
    (bind _output_get (Variables|Default|SetHolding (not (stale _output_get)))))
  (for _array_element (Variables|Default|GetActivables)
    (Class|InteractInterfaceBP|TriggerActivator(Message) _array_element (Variables|Default|GetChannel)))
  (CallFunction|EventLightUp))

(event Custom|Event%20LightUp
  ;[1 1 1] Interface Events
  (if (Variables|Default|GetHold)
    (Rendering|Material|SetMaterial (Variables|Default|GetActivatorMesh) 3 (Utilities|Array|Get(acopy) (Utilities|Array|MakeArray "/Game/Arte/Materials/02_default_Tramp.02_default_Tramp" "/Game/Arte/Materials/02_default_Tramp_I_Blue.02_default_Tramp_I_Blue") (Math|Integer|SelectInt 0 1 (Variables|Default|GetHolding))))))

(event EventToggleWidget
  ;[1 1 1] Interface Events
  (Rendering|SetVisibility (Variables|Default|GetInteractionWidget) true false)
  (Utilities|FlowControl|RetriggerableDelay 0.2)
  (Rendering|SetVisibility (Variables|Default|GetInteractionWidget) false false))

(event EventTelekinesisEffectUpdate
  (params (Channel :type Integer))
  (bind _variable (|TemporaryVariable))
  (bind _activatormesh (Variables|Default|GetActivatorMesh))
  (Utilities|FlowControl|Sequence
    (:then_0
      (if (!= Channel _variable)
        (goto _label Reset)))
    (:then_1
      (Utilities|FlowControl|DoOnce false :!label _label
        (:Completed
          (Rendering|SetRenderCustomDepth _activatormesh true)
          (Rendering|SetCustomDepthStencilValue _activatormesh Channel)
          (|Assign _variable Channel))))
    (:then_2
      (Utilities|FlowControl|RetriggerableDelay 0.3)
      (Rendering|SetRenderCustomDepth (Variables|Default|GetActivatorMesh) false)
      (goto _label Reset))))

(event EventTelekinesisBegin
  (params (Rafi :type Pawn%20Object%20Reference) (H%20range :type Float%20%28single-precision%29) (V%20Range :type Float%20%28single-precision%29))
  ;[1 1 1] Interface Events
  (Variables|Default|SetRafi Rafi))

(event EventTelekinesisEnd
  (params (Rafi :type Pawn%20Object%20Reference))
  ;[1 1 1] Interface Events
  (Variables|Default|SetRafi 0))

(fn ConstructionScript
  (bind _telekinesiscomponent (Variables|Default|GetTelekinesisComponent))
  (if (Variables|Default|GetTelekinesis)
    (Collision|SetCollisionEnabled _telekinesiscomponent "QueryOnly")
    (else
      (Collision|SetCollisionEnabled _telekinesiscomponent "NoCollision"))))

(fn Interact
  (params (Telekinesis :type Boolean))
  (if Telekinesis
    (if (Variables|Default|GetTelekinesis)
      (CallFunction|EventActivate :!label _label)
      (return (Variables|Default|GetHold)))
    (else
      (goto _label))))

(fn TelekinesisCameraOffset
  (return 0.0))

(fn TelekinesisPileUp
  (params (Input :type Array%20of%20Actor%20Object%20References))
  (return 0))