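; Base door Blueprint that opens and closes through activator interface events for interaction, trigger, unlock and widget toggling.
; Interact respects the lock, while trigger bypasses it; both share a DoOnce that plays or reverses the DoorMovement timeline and resets when it finishes.
; The timeline feeds alpha to AnimateDoor, an empty event here, which the construction script also calls to pose doors that start open.
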(event Custom|Animate%20Door
  (params (Alpha :type Float%20%28single-precision%29))
  ;[1 1 1] Door Animation
)

(event EventToggleWidget
  (params (Visible :type Boolean))
  ;[1 1 1] Interface Events
  (if (not (Variables|Default|GetLocked))
    (Rendering|SetVisibility (Variables|Default|GetInteractionWidget) Visible false)))

(event EventUnlockActivator
  ;[1 1 1] Interface Events
  (Variables|Default|SetLocked false))

(event EventTriggerActivator
  ;[1 1 1] Interface Events
  (Utilities|FlowControl|DoOnce false :!label _label
    (:Completed
      (if (Variables|Default|GetClosed)
        (bind _alpha (Timeline|Door%20Movement PlayFromStart)
          (:Update
            (CallFunction|AnimateDoor _alpha))
          (:Finished
            (bind _output_get (Variables|Default|SetClosed (not (stale _output_get))))
            (goto _label Reset)))
        (else
          (Timeline|Door%20Movement ReverseFromEnd))))))

(event EventInteractActivator
  ;[1 1 1] Interface Events
  (if (not (Variables|Default|GetLocked))
    (Utilities|FlowControl|DoOnce false :!label _label
      (:Completed
        (if (Variables|Default|GetClosed)
          (bind _alpha (Timeline|Door%20Movement PlayFromStart)
            (:Update
              (CallFunction|AnimateDoor _alpha))
            (:Finished
              (bind _output_get (Variables|Default|SetClosed (not (stale _output_get))))
              (goto _label Reset)))
          (else
            (Timeline|Door%20Movement ReverseFromEnd)))))))

(fn ConstructionScript
  (if (not (Variables|Default|GetClosed))
    (CallFunction|AnimateDoor 1.0)))